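; Potion of Fortune is a usable potion actor that grants the player's GoblinCharacter a temporary Fortune effect.
; Its Use event sets the character's Fortune flag, marks itself active and shows the character's PotionOfFortune component.
; After a 30-second delay it hides that component, clears both flags and destroys itself.
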(event `self.Use`
  (bind _asgoblin_character (cast `/Game/Blueprints/GoblinCharacter` (`GameplayStatics.GetPlayerCharacter` 0)))
  (set `/Game/Blueprints/GoblinCharacter.Fortune` true _asgoblin_character)
  (set `self.IsActive` true)
  (bind _potionoffortune (`/Game/Blueprints/GoblinCharacter.PotionOfFortune` _asgoblin_character))
  (`SceneComponent.SetVisibility` _potionoffortune true false)
  (`KismetSystemLibrary.Delay` 30.0)
  (`SceneComponent.SetVisibility` _potionoffortune false false)
  (set `/Game/Blueprints/GoblinCharacter.Fortune` false _asgoblin_character)
  (set `self.IsActive` false)
  (`self.K2_DestroyActor`))

(fn `UserConstructionScript`
  (`parent.UserConstructionScript`))