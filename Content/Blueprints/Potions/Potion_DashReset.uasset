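; Potion Blueprint that resets the player's dash in the game when used.
; Use casts player character 0 to GoblinCharacter and sets its Dashcounter to its Dashcooldown value.
; It then plays a 2D drinking sound, holds IsActive true for one second, and destroys itself.
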(event `self.Use`
  (bind _asgoblin_character (cast `/Game/Blueprints/GoblinCharacter` (`GameplayStatics.GetPlayerCharacter` 0)))
  (set `/Game/Blueprints/GoblinCharacter.Dashcounter` (`/Game/Blueprints/GoblinCharacter.Dashcooldown` _asgoblin_character) _asgoblin_character)
  (`GameplayStatics.PlaySound2D` "/Game/Sounds/Effects/potion_drink.potion_drink" 1.0 1.0 0.0 null null)
  (set `self.IsActive` true)
  (`KismetSystemLibrary.Delay` 1.0)
  (set `self.IsActive` false)
  (`self.K2_DestroyActor`))

(fn `UserConstructionScript`
  (`parent.UserConstructionScript`))