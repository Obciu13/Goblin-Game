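; Health potion actor that restores one HP to the player's GoblinCharacter when used.
; Its Use event casts player 0's character and checks HP against MaxHP.
; Below max, it adds the HP, holds IsActive true for a one-second delay, then destroys itself.
; At full health, it only prints a Polish "full health" message and remains in place.
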(event `self.Use`
  (bind _asgoblin_character (cast `/Game/Blueprints/GoblinCharacter` (`GameplayStatics.GetPlayerCharacter` 0)))
  (bind _hp (`/Game/Blueprints/GoblinCharacter.HP` _asgoblin_character))
  (if (< _hp (`/Game/Blueprints/GoblinCharacter.MaxHP` _asgoblin_character))
    (set `self.IsActive` true)
    (set `/Game/Blueprints/GoblinCharacter.HP` (+ _hp 1.0) _asgoblin_character)
    (`KismetSystemLibrary.Delay` 1.0)
    (set `self.IsActive` false)
    (`self.K2_DestroyActor`)
    (else
      (`KismetSystemLibrary.PrintString` "Masz pelne zycie"))))

(fn `UserConstructionScript`
  (`parent.UserConstructionScript`))