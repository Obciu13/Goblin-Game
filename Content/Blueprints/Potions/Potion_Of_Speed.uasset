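; Potion of Speed is a potion actor that temporarily boosts the player goblin's walk speed when used.
; Its Use event casts player character 0 to GoblinCharacter, raises max walk speed and sets IsActive for a ten-second delay.
; It then clears the flag, resets speed to a hardcoded value rather than the previous one, and destroys itself.
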(event `self.Use`
  (bind _asgoblin_character (cast `/Game/Blueprints/GoblinCharacter` (`GameplayStatics.GetPlayerCharacter` 0)))
  (bind _charactermovement (`Character.CharacterMovement` _asgoblin_character))
  (set `CharacterMovementComponent.MaxWalkSpeed` 1000.0 _charactermovement)
  (set `self.IsActive` true)
  (`KismetSystemLibrary.Delay` 10.0)
  (set `self.IsActive` false)
  (set `CharacterMovementComponent.MaxWalkSpeed` 600.0 _charactermovement)
  (`self.K2_DestroyActor`))

(fn `UserConstructionScript`
  (`parent.UserConstructionScript`))