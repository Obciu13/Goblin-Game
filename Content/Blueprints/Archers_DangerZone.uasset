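; Danger zone volume that rains area-of-effect arrow attacks around the player while the goblin character is inside its box.
; Severity sets the repeat delay of a looping timer that starts on overlap, pauses on exit and resumes on re-entry; zero disables it.
; Each volley spawns randomly staggered AOE_Arrows at scattered points ahead of the player with random yaw, adding a third at the highest severity.
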(event `self.ReceiveBeginPlay`
  ;[1 1 1] Set Delay
  (switch `int` (`self.Severity`)
    (:`1`
      (set `self.Delay` 4.0))
    (:`2`
      (set `self.Delay` 3.0))
    (:`3`
      (set `self.Delay` 2.0))))

(event `self.Box.OnComponentBeginOverlap`
  (params (OverlappedComponent :type "PrimitiveComponent Object Reference") (OtherActor :type "Actor Object Reference") (OtherComp :type "PrimitiveComponent Object Reference") (OtherBodyIndex :type Integer) (bFromSweep :type Boolean) (SweepResult :type "HitResult Structure (by ref)"))
  ;[1 1 1] On Goblin Overlap
  (cast `/Game/Blueprints/GoblinCharacter` OtherActor)
  (set `self.Player in Range` true)
  (if (!= (`self.Severity`) 0)
    (if (`KismetSystemLibrary.K2_IsValidTimerHandle` (`self.Handle`))
      (`KismetSystemLibrary.K2_UnPauseTimerHandle` (`self.Handle`))
      (else
        (bind _returnvalue (`KismetSystemLibrary.K2_SetTimerDelegate` (delegate `CustomEvent_0`) (`self.Delay`) true (`self.Initial Delay`)))
        (set `self.Handle` _returnvalue)))))

(event `CustomEvent_0`
  ;[1 1 1] On Goblin Overlap
  (bind _returnvalue (`self.Aim For Player` 1000.0))
  (`|SpawnActorFromClass` "/Game/Blueprints/Skillshots/AOE_Arrows.AOE_Arrows_C" _returnvalue "Undefined" "OverrideRootScale" null null)
  (`KismetSystemLibrary.Delay` (`KismetMathLibrary.RandomFloat`))
  (bind _returnvalue_2 (`self.Aim For Player` 300.0))
  (`|SpawnActorFromClass` "/Game/Blueprints/Skillshots/AOE_Arrows.AOE_Arrows_C" _returnvalue_2 "Undefined" "OverrideRootScale" null null)
  (if (== (`self.Severity`) 3)
    (`KismetSystemLibrary.Delay` (`KismetMathLibrary.RandomFloat`))
    (bind _returnvalue_3 (`self.Aim For Player` 400.0))
    (`|SpawnActorFromClass` "/Game/Blueprints/Skillshots/AOE_Arrows.AOE_Arrows_C" _returnvalue_3 "Undefined" "OverrideRootScale" null null)))

(event `self.Box.OnComponentEndOverlap`
  (params (OverlappedComponent :type "PrimitiveComponent Object Reference") (OtherActor :type "Actor Object Reference") (OtherComp :type "PrimitiveComponent Object Reference") (OtherBodyIndex :type Integer))
  ;[1 1 1] On Goblin End Overlap
  (cast `/Game/Blueprints/GoblinCharacter` OtherActor)
  (set `self.Player in Range` false)
  (if (`KismetSystemLibrary.K2_IsValidTimerHandle` (`self.Handle`))
    (`KismetSystemLibrary.K2_PauseTimerHandle` (`self.Handle`))))

(fn `Aim for Player`
  (params (Variance :type "Float (double-precision)"))
  (returns (ReturnValue :type "Transform Structure"))
  (bind _returnvalue (`GameplayStatics.GetPlayerCharacter` 0))
  (return (`KismetMathLibrary.MakeTransform` (+ (`self.K2_GetActorLocation` _returnvalue) (* (`self.GetActorForwardVector` _returnvalue) (`KismetMathLibrary.FTrunc` (`self.Distance from Character`))) (`KismetMathLibrary.MakeVector` (`KismetMathLibrary.RandomFloatInRange` (* Variance -1.0) Variance) (`KismetMathLibrary.RandomFloatInRange` (* Variance -1.0) Variance) 70.0)) (`KismetMathLibrary.MakeRotator` 0.0 0.0 (`KismetMathLibrary.RandomFloatInRange` 0.0 360.0)))))

(fn `UserConstructionScript`)