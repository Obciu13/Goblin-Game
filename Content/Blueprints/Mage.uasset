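; Mage enemy that attacks the goblin player with random area-of-effect spells while they are inside its detection sphere.
; Sphere overlaps start, pause and resume a looping timer that calls CastSpell, which turns the mage toward the player and picks a spell.
; Fireball and meteor rain target random reachable points near the player, Pull spawns above the mage, and Wave steps toward the player's saved position.
; Meteor rain and Wave repeat through delayed, counter-limited self-calls.
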(event `self.ReceiveBeginPlay`
  (`SceneComponent.K2_SetWorldTransform` (`self.staff`) (`SceneComponent.GetSocketTransform` (`self.SkeletalMesh`) "Hold" "RTS_World") false false)
  (`SceneComponent.K2_AttachToComponent` (`self.staff`) (`self.SkeletalMesh`) "Hold" "SnapToTarget" "SnapToTarget" "SnapToTarget" true))

(event `Rotate to face player`
  (bind (_returnvalue_roll _returnvalue_pitch _returnvalue_yaw) (`KismetMathLibrary.BreakRotator` (`KismetMathLibrary.FindLookAtRotation` (`self.K2_GetActorLocation`) (`self.K2_GetActorLocation` (`GameplayStatics.GetPlayerCharacter` 0)))))
  ;[1 1 1] Rotate To face Player
  (`SceneComponent.K2_SetWorldRotation` (`self.SkeletalMesh`) (`KismetMathLibrary.MakeRotator` 0.0 0.0 (+ _returnvalue_yaw -90.0)) false false))

(event `self.Sphere.OnComponentBeginOverlap`
  (params (OverlappedComponent :type "PrimitiveComponent Object Reference") (OtherActor :type "Actor Object Reference") (OtherComp :type "PrimitiveComponent Object Reference") (OtherBodyIndex :type Integer) (bFromSweep :type Boolean) (SweepResult :type "HitResult Structure (by ref)"))
  ;[1 1 1] Overlap
  (cast `/Game/Blueprints/GoblinCharacter` OtherActor)
  (set `self.Player in Range` true)
  (if (`KismetSystemLibrary.K2_IsValidTimerHandle` (`self.Timer`))
    (`KismetSystemLibrary.K2_UnPauseTimerHandle` (`self.Timer`))
    (else
      (`self.CastSpell`)
      (bind _returnvalue (`KismetSystemLibrary.K2_SetTimer` null "CastSpell" 8.0 true))
      (set `self.Timer` _returnvalue))))

(event `self.Sphere.OnComponentEndOverlap`
  (params (OverlappedComponent :type "PrimitiveComponent Object Reference") (OtherActor :type "Actor Object Reference") (OtherComp :type "PrimitiveComponent Object Reference") (OtherBodyIndex :type Integer))
  (bind _timer (`self.Timer`))
  ;[1 1 1] Overlap
  (cast `/Game/Blueprints/GoblinCharacter` OtherActor)
  (set `self.Player in Range` false)
  (if (`KismetSystemLibrary.K2_IsValidTimerHandle` _timer)
    (`KismetSystemLibrary.K2_PauseTimerHandle` _timer)))

(event `Fireball`
  (bind _returnvalue (`self.K2_GetActorLocation` (`GameplayStatics.GetPlayerCharacter` 0)))
  (bind _randomlocation (`NavigationSystemV1.K2_GetRandomReachablePointInRadius` _returnvalue 100.0 null null))
  ;[1 1 1] Fireball
  (`/Engine/EditorBlueprintResources/StandardMacros.IncrementInt` (`self.Counter`)
    (:`  `
      (`KismetSystemLibrary.Delay` 0.5)
      (`|SpawnActorFromClass` "/Game/Blueprints/Skillshots/AOE_Fireball.AOE_Fireball_C" (`KismetMathLibrary.Conv_VectorToTransform` (`KismetMathLibrary.MakeVector` (.x _randomlocation) (.y _randomlocation) (+ (.z _returnvalue) 50.0))) "Undefined" "OverrideRootScale" null null)
      (`SkeletalMeshComponent.PlayAnimation` (`self.SkeletalMesh`) "/Game/Animations/Mage/Lowpoly_mage_Anim_Mage_Szkielet_MageSummonShort_Animation.Lowpoly_mage_Anim_Mage_Szkielet_MageSummonShort_Animation" false)
      (`GameplayStatics.PlaySound2D` "/Game/Sounds/Effects/New_Sounds/firewush.firewush" 1.0 1.0 0.0 null null)
      (`KismetSystemLibrary.Delay` 1.0)
      (`GameplayStatics.PlaySound2D` "/Game/StarterContent/Audio/Explosion01.Explosion01" 1.0 1.0 0.0 null null))))

(event `Pull`
  ;[1 1 1] Pull
  (`|SpawnActorFromClass` "/Game/Blueprints/Skillshots/AOE_Pull.AOE_Pull_C" (`KismetMathLibrary.MakeTransform` (`KismetMathLibrary.MakeVector` (.x (.location (`self.GetTransform`))) (.y (.location (`self.GetTransform`))) (+ (.z (.location (`self.GetTransform`))) 120.0))) "Undefined" "OverrideRootScale" null null)
  (`GameplayStatics.PlaySound2D` "/Game/Sounds/Effects/New_Sounds/Trap_sound.Trap_sound" 1.0 1.0 0.0 null null)
  (`KismetSystemLibrary.Delay` 1.0)
  (`SkeletalMeshComponent.PlayAnimation` (`self.SkeletalMesh`) "/Game/Animations/Mage/Lowpoly_mage_Anim_Mage_Szkielet_MageSummon_Animation.Lowpoly_mage_Anim_Mage_Szkielet_MageSummon_Animation" false)
  (`KismetSystemLibrary.Delay` 1.7)
  (`GameplayStatics.PlaySound2D` "/Game/Sounds/Effects/New_Sounds/Shield.Shield" 1.0 1.0 0.0 null null))

(event `Meteors rain`
  (bind _returnvalue (`self.K2_GetActorLocation` (`GameplayStatics.GetPlayerCharacter` 0)))
  (bind _randomlocation (`NavigationSystemV1.K2_GetRandomReachablePointInRadius` _returnvalue 100.0 null null))
  ;[1 1 1] Meteor rains
  (`/Engine/EditorBlueprintResources/StandardMacros.IncrementInt` (`self.Counter`)
    (:`  `
      (`KismetSystemLibrary.Delay` 0.5)
      (`|SpawnActorFromClass` "/Game/Blueprints/Skillshots/AOE_Meteor.AOE_Meteor_C" (`KismetMathLibrary.Conv_VectorToTransform` (`KismetMathLibrary.MakeVector` (.x _randomlocation) (.y _randomlocation) (+ (.z _returnvalue) 50.0))) "Undefined" "OverrideRootScale" null null)
      (`GameplayStatics.PlaySound2D` "/Game/Sounds/Effects/New_Sounds/firewush.firewush" 1.0 1.0 0.0 null null)
      (if (<= (`self.Counter`) 5)
        (`self.Meteors rain`)
        (if (== (`self.Counter`) 1)
          (`SkeletalMeshComponent.PlayAnimation` (`self.SkeletalMesh`) "/Game/Animations/Mage/Lowpoly_mage_Anim_Mage_Szkielet_MageCast_Animation.Lowpoly_mage_Anim_Mage_Szkielet_MageCast_Animation" false))))))

(event `Wave`
  (bind _returnvalue (`self.K2_GetActorLocation`))
  (bind _returnvalue_2 (`KismetMathLibrary.GetDirectionUnitVector` _returnvalue (`self.Target location`)))
  ;[1 1 1] Wave
  (`/Engine/EditorBlueprintResources/StandardMacros.IncrementInt` (`self.Counter`)
    (:`  `
      (`|SpawnActorFromClass` "/Game/Blueprints/Skillshots/AOE_Wave.AOE_Wave_C" (`KismetMathLibrary.MakeTransform` (`KismetMathLibrary.MakeVector` (.x (+ (* (* _returnvalue_2 300) (`self.Counter`)) _returnvalue)) (.y (+ (* (* _returnvalue_2 300) (`self.Counter`)) _returnvalue)) (+ (.z (`self.K2_GetActorLocation` (`GameplayStatics.GetPlayerCharacter` 0))) 50.0)) (`KismetMathLibrary.Quat_Rotator` (`KismetMathLibrary.Conv_VectorToQuaternion` _returnvalue_2))) "Undefined" "OverrideRootScale" null null)
      (`GameplayStatics.PlaySound2D` "/Game/Sounds/Effects/New_Sounds/firewush.firewush" 1.0 1.0 0.0 null null)
      (`KismetSystemLibrary.Delay` 0.2)
      (if (<= (`self.Counter`) 5)
        (`self.Wave`)
        (if (== (`self.Counter`) 1)
          (`SkeletalMeshComponent.PlayAnimation` (`self.SkeletalMesh`) "/Game/Animations/Mage/Lowpoly_mage_Anim_Mage_Szkielet_MageFastCast_Animation.Lowpoly_mage_Anim_Mage_Szkielet_MageFastCast_Animation" false))))))

(fn `CastSpell`
  (if (`self.Player in Range`)
    (`self.Rotate to face player`)
    (switch `int` (`KismetMathLibrary.RandomIntegerInRange` 0 3)
      (:`0`
        (`self.Meteors rain`))
      (:`1`
        (`self.Fireball`))
      (:`2`
        (set `self.Target location` (`self.K2_GetActorLocation` (`GameplayStatics.GetPlayerCharacter` 0)))
        (`self.Wave`))
      (:`3`
        (`self.Pull`)))
    (set `self.Counter` 0)))

(fn `UserConstructionScript`)