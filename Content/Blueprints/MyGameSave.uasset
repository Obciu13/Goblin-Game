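; MyGameSave is a save-data Blueprint that holds player progression: gold, max HP, upgrade levels, drop chances, potion class, tutorial state and game phase.
; SaveVariablesfromInstance copies these values from the Game Instance into its own variables, and LoadtoInstance copies them back.
; Max HP is truncated to an integer on save, so any fractional part is lost.
; Writing to and reading from a save slot happens outside this graph.
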(event `Save Variables from Instance`
  (params (`Game Instance` :type "/Game/Blueprints/MyGameInstance Object Reference"))
  (set `self.Gameinstance` `Game Instance`)
  (set `self.Player_Gold` (`/Game/Blueprints/MyGameInstance.Gold` (`self.Gameinstance`)))
  (set `self.Player_MaxHp` (`KismetMathLibrary.FTrunc` (`/Game/Blueprints/MyGameInstance.MaxHp` (`self.Gameinstance`))))
  (set `self.Player_GoldSniffingLevel` (`/Game/Blueprints/MyGameInstance.GoldSniffingLevel` (`self.Gameinstance`)))
  (set `self.Player_GoldDropChance` (`/Game/Blueprints/MyGameInstance.Gold_Drop_Chance` (`self.Gameinstance`)))
  (set `self.Player_PotionDropChance` (`/Game/Blueprints/MyGameInstance.Potion_Drop_Chance` (`self.Gameinstance`)))
  (set `self.Player_TenacityLevel` (`/Game/Blueprints/MyGameInstance.Tenacity Level` (`self.Gameinstance`)))
  (set `self.Player_PotionClass` (`/Game/Blueprints/MyGameInstance.PotionClass` (`self.Gameinstance`)))
  (set `self.Player_CaravanScourgeLevel` (`/Game/Blueprints/MyGameInstance.CaravanScourge Level` (`self.Gameinstance`)))
  (set `self.Player_MagicGadgetMasterLevel` (`/Game/Blueprints/MyGameInstance.MagicGadgetMaster Level` (`self.Gameinstance`)))
  (set `self.Player_DurabilityLevel` (`/Game/Blueprints/MyGameInstance.Durability Level` (`self.Gameinstance`)))
  (set `self.Player_CorpseRobberGoldLevel` (`/Game/Blueprints/MyGameInstance.CorpseRobberGold Level` (`self.Gameinstance`)))
  (set `self.Player_CorpseRobberPotionLevel` (`/Game/Blueprints/MyGameInstance.CorpseRobberPotion Level` (`self.Gameinstance`)))
  (set `self.Player_AlchemistLevel` (`/Game/Blueprints/MyGameInstance.Alchemist_Level` (`self.Gameinstance`)))
  (set `self.Tutorial` (`/Game/Blueprints/MyGameInstance.Tutorial` (`self.Gameinstance`)))
  (set `self.Gold_Given` (`/Game/Blueprints/MyGameInstance.Gold_Given` (`self.Gameinstance`)))
  (set `self.GamePhase` (`/Game/Blueprints/MyGameInstance.Game Phase` (`self.Gameinstance`))))

(event `Load to Instance`
  (params (Instance :type "/Game/Blueprints/MyGameInstance Object Reference"))
  (set `self.Gameinstance` Instance)
  (set `/Game/Blueprints/MyGameInstance.Gold` (`self.Player_Gold`) (`self.Gameinstance`))
  (set `/Game/Blueprints/MyGameInstance.MaxHp` (`KismetMathLibrary.Conv_IntToDouble` (`self.Player_MaxHp`)) (`self.Gameinstance`))
  (set `/Game/Blueprints/MyGameInstance.GoldSniffingLevel` (`self.Player_GoldSniffingLevel`) (`self.Gameinstance`))
  (set `/Game/Blueprints/MyGameInstance.Gold_Drop_Chance` (`self.Player_GoldDropChance`) (`self.Gameinstance`))
  (set `/Game/Blueprints/MyGameInstance.Potion_Drop_Chance` (`self.Player_PotionDropChance`) (`self.Gameinstance`))
  (set `/Game/Blueprints/MyGameInstance.Tenacity Level` (`self.Player_TenacityLevel`) (`self.Gameinstance`))
  (set `/Game/Blueprints/MyGameInstance.PotionClass` (`self.Player_PotionClass`) (`self.Gameinstance`))
  (set `/Game/Blueprints/MyGameInstance.CaravanScourge Level` (`self.Player_CaravanScourgeLevel`) (`self.Gameinstance`))
  (set `/Game/Blueprints/MyGameInstance.Durability Level` (`self.Player_DurabilityLevel`) (`self.Gameinstance`))
  (set `/Game/Blueprints/MyGameInstance.CorpseRobberGold Level` (`self.Player_CorpseRobberGoldLevel`) (`self.Gameinstance`))
  (set `/Game/Blueprints/MyGameInstance.CorpseRobberPotion Level` (`self.Player_CorpseRobberPotionLevel`) (`self.Gameinstance`))
  (set `/Game/Blueprints/MyGameInstance.MagicGadgetMaster Level` (`self.Player_MagicGadgetMasterLevel`) (`self.Gameinstance`))
  (set `/Game/Blueprints/MyGameInstance.Alchemist_Level` (`self.Player_AlchemistLevel`) (`self.Gameinstance`))
  (set `/Game/Blueprints/MyGameInstance.Tutorial` (`self.Tutorial`) (`self.Gameinstance`))
  (set `/Game/Blueprints/MyGameInstance.Gold_Given` (`self.Gold_Given`) (`self.Gameinstance`))
  (set `/Game/Blueprints/MyGameInstance.Game Phase` (`self.GamePhase`) (`self.Gameinstance`)))