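; Dragon fire area-of-effect skillshot actor that scales its effect, plays a fire sound and destroys itself after 20 seconds.
; Sphere overlap flags a GoblinCharacter as the player in range and starts Burn, which re-triggers itself every half second while that flag holds.
; Burn calls DealDamage on the player and damages every AI in HIttedAI, a list this graph never fills.
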(event `self.ReceiveBeginPlay`
  (`self.Scale_effect`)
  (`GameplayStatics.SpawnSoundAtLocation` "/Game/StarterContent/Audio/Fire01_Cue.Fire01_Cue" (`self.K2_GetActorLocation`) (struct) 0.5 1.0 0.0 null null)
  (`KismetSystemLibrary.Delay` 20.0)
  (`self.K2_DestroyActor`))

(event `Burn`
  (`|ExecutionSequence`
    (:`then_0`
      ;[1 1 1] Player
      (if (`self.Player in range`)
        (`self.Deal damage`)
        (`KismetSystemLibrary.Delay` 0.5 :!label _label)
        (if (`self.Player in range`)
          (`self.Burn`))))
    (:`then_1`
      ;[1 1 1] AI
      (for _array_element (`self.HIttedAI`)
        (`/Game/AI2/EnemyCharacter.Get damage` _array_element 5.0)
        (goto _label)))))

(event `self.Sphere.OnComponentBeginOverlap`
  (params (OverlappedComponent :type "PrimitiveComponent Object Reference") (OtherActor :type "Actor Object Reference") (OtherComp :type "PrimitiveComponent Object Reference") (OtherBodyIndex :type Integer) (bFromSweep :type Boolean) (SweepResult :type "HitResult Structure (by ref)"))
  (cast `/Game/Blueprints/GoblinCharacter` OtherActor)
  (set `self.Player in range` true)
  (`self.Burn`))

(event `self.Sphere.OnComponentEndOverlap`
  (params (OverlappedComponent :type "PrimitiveComponent Object Reference") (OtherActor :type "Actor Object Reference") (OtherComp :type "PrimitiveComponent Object Reference") (OtherBodyIndex :type Integer))
  (cast `/Game/Blueprints/GoblinCharacter` OtherActor)
  (set `self.Player in range` false))

(fn `UserConstructionScript`
  (`parent.UserConstructionScript`))