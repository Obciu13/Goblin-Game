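; Dragon breath skillshot actor that spawns a radial burst of AOE_DragonFire actors, then destroys itself.
; On BeginPlay it takes a random yaw, waits briefly, and spawns a larger fire at the central Cylinder.
; Burning then spawns small fires at each "Fire"-tagged mesh, stepping those meshes outward from the center in timed waves.
; Each outward wave's fires spawn one further step beyond the moved mesh.
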(event `self.ReceiveBeginPlay`
  (set `self.Fires` (`self.GetComponentsByTag` "/Script/Engine.StaticMeshComponent" "Fire"))
  (`self.K2_SetActorRotation` (`KismetMathLibrary.MakeRotator` 0.0 0.0 (`KismetMathLibrary.RandomFloatInRange` 0.0 360.0)))
  (`KismetSystemLibrary.Delay` 1.0)
  (`|SpawnActorFromClass` "/Game/Blueprints/Skillshots/AOE_DragonFire.AOE_DragonFire_C" (`KismetMathLibrary.MakeTransform` (`SceneComponent.K2_GetComponentLocation` (`self.Cylinder`))) "Undefined" "OverrideRootScale" null (0.3 0.3 0.3) null)
  (`KismetSystemLibrary.Delay` 0.1)
  (`self.Burning`))

(event `Burning`
  ;[1 1 1] Burning
  (for _array_element (`self.Fires`)
    (`|SpawnActorFromClass` "/Game/Blueprints/Skillshots/AOE_DragonFire.AOE_DragonFire_C" (`KismetMathLibrary.MakeTransform` (`SceneComponent.K2_GetComponentLocation` _array_element) (`KismetMathLibrary.MakeRotator` 0.0)) "Undefined" "OverrideRootScale" null (0.1 0.1 0.1) null))
  (`KismetSystemLibrary.Delay` 0.1)
  (for _array_element_2 (`self.Fires`)
    (bind _returnvalue (`SceneComponent.K2_GetComponentLocation` _array_element_2))
    (bind _returnvalue_2 (+ _returnvalue (* (`KismetMathLibrary.GetDirectionUnitVector` (`SceneComponent.K2_GetComponentLocation` (`self.Cylinder`)) _returnvalue) 100.0)))
    (`SceneComponent.K2_SetWorldLocation` _array_element_2 _returnvalue_2 false true)
    (`|SpawnActorFromClass` "/Game/Blueprints/Skillshots/AOE_DragonFire.AOE_DragonFire_C" (`KismetMathLibrary.MakeTransform` _returnvalue_2 (`KismetMathLibrary.MakeRotator` 0.0)) "Undefined" "OverrideRootScale" null (0.1 0.1 0.1) null))
  (`KismetSystemLibrary.Delay` 0.1)
  (for _array_element_3 (`self.Fires`)
    (bind _returnvalue_3 (`SceneComponent.K2_GetComponentLocation` _array_element_3))
    (bind _returnvalue_4 (+ _returnvalue_3 (* (`KismetMathLibrary.GetDirectionUnitVector` (`SceneComponent.K2_GetComponentLocation` (`self.Cylinder`)) _returnvalue_3) 150.0)))
    (`SceneComponent.K2_SetWorldLocation` _array_element_3 _returnvalue_4 false true)
    (`|SpawnActorFromClass` "/Game/Blueprints/Skillshots/AOE_DragonFire.AOE_DragonFire_C" (`KismetMathLibrary.MakeTransform` _returnvalue_4 (`KismetMathLibrary.MakeRotator` 0.0)) "Undefined" "OverrideRootScale" null (0.1 0.1 0.1) null))
  (`KismetSystemLibrary.Delay` 0.1)
  (for _array_element_4 (`self.Fires`)
    (bind _returnvalue_5 (`SceneComponent.K2_GetComponentLocation` _array_element_4))
    (bind _returnvalue_6 (+ _returnvalue_5 (* (`KismetMathLibrary.GetDirectionUnitVector` (`SceneComponent.K2_GetComponentLocation` (`self.Cylinder`)) _returnvalue_5) 150.0)))
    (`SceneComponent.K2_SetWorldLocation` _array_element_4 _returnvalue_6 false true)
    (`|SpawnActorFromClass` "/Game/Blueprints/Skillshots/AOE_DragonFire.AOE_DragonFire_C" (`KismetMathLibrary.MakeTransform` _returnvalue_6 (`KismetMathLibrary.MakeRotator` 0.0)) "Undefined" "OverrideRootScale" null (0.1 0.1 0.1) null))
  (`KismetSystemLibrary.Delay` 0.5)
  (`self.K2_DestroyActor`))

(fn `UserConstructionScript`)