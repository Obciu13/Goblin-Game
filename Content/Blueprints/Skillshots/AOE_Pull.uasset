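; Skillshot area-of-effect actor that grows in while spinning, then bursts and pulls characters.
; BeginPlay runs a scale timeline whose Update leads through delays to stop the spin, spawn particles, call Pull and destroy the actor.
; Pull impulses an in-range player goblin toward the center; otherwise it impulses HIttedAI, using a force derived from the unset goblin cast rather than each AI's location.
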(event `self.ReceiveBeginPlay`
  (bind _returnvalue (`AddComponent|NODE_AddRotatingMovementComponent-0`))
  (set `RotatingMovementComponent.RotationRate` (struct :`Yaw` 100.0) _returnvalue)
  (bind (_direction _growtrack) (`Timeline|Grow Timeline` :!via `PlayFromStart`)
    (:`Update`
      (`self.SetActorScale3D` _growtrack)
      (`KismetSystemLibrary.Delay` (`self.Delay`))
      (`ActorComponent.K2_DestroyComponent` _returnvalue)
      (set `self.StopSpinning` true)
      (`KismetSystemLibrary.Delay` 1.0)
      (bind _returnvalue_2 (`GameplayStatics.SpawnEmitterAtLocation` (`self.Particle System`) (`self.K2_GetActorLocation`) (struct) (* (`self.Scale`) 2)))
      (`self.Pull`)
      (`KismetSystemLibrary.Delay` 0.2)
      (`ActorComponent.K2_DestroyComponent` _returnvalue_2)
      (`self.K2_DestroyActor`))))

(fn `Pull`
  (if (`self.Player in range`)
    (bind _asgoblin_character (cast `/Game/Blueprints/GoblinCharacter` (`GameplayStatics.GetPlayerCharacter` 0))
      (:`then`
        (bind _output_get (set `self.Force` (- (`self.K2_GetActorLocation` _asgoblin_character) (`self.K2_GetActorLocation`))))
        (`CharacterMovementComponent.AddImpulse` (`Character.CharacterMovement` _asgoblin_character) (* _output_get -3) true))
      (:`CastFailed`
        (for _array_element (`self.HIttedAI`) :!label _label
          (bind _output_get_2 (set `self.Force` (- (`self.K2_GetActorLocation`) (`self.K2_GetActorLocation` _asgoblin_character))))
          (`CharacterMovementComponent.AddImpulse` (`Character.CharacterMovement` _array_element) _output_get_2 false))))
    (else
      (goto _label))))

(fn `UserConstructionScript`
  (`parent.UserConstructionScript`))