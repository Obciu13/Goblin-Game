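; Tornado area-of-effect skillshot that chases the player goblin for eight seconds as its sound fades, then destroys itself.
; A looping one-second timer re-aims it at the player, sets forward speed scaled by player level, and calls Burn.
; Burn damages the player inside the sphere and every AI in HIttedAI, which is not filled here.
; A half-second delay repeats Burn while the player stays inside.
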(event `self.ReceiveBeginPlay`
  ;[1 1 1] Begin Play
  (bind _asgoblin_character (cast `/Game/Blueprints/GoblinCharacter` (`GameplayStatics.GetPlayerCharacter` 0)))
  (set `self.Speed` (+ (* (/ (`/Game/Blueprints/GoblinCharacter.Level` _asgoblin_character) 6) 30.0) 200.0))
  (`self.Scale_effect`)
  (`KismetSystemLibrary.K2_SetTimer` null "Chase" 1.0 true)
  (bind _returnvalue (`GameplayStatics.SpawnSoundAttached` "/Game/Fire02_Cue.Fire02_Cue" (`self.Niagara`) "None" (0.0 0.0 0.0) (struct) "KeepRelativeOffset" true 1.0 1.0 0.0 null null))
  (`AudioComponent.AdjustVolume` _returnvalue 8.0 0.0 "Linear")
  (`KismetSystemLibrary.Delay` 8.0)
  (`self.K2_DestroyActor`))

(event `self.Sphere.OnComponentBeginOverlap`
  (params (OverlappedComponent :type "PrimitiveComponent Object Reference") (OtherActor :type "Actor Object Reference") (OtherComp :type "PrimitiveComponent Object Reference") (OtherBodyIndex :type Integer) (bFromSweep :type Boolean) (SweepResult :type "HitResult Structure (by ref)"))
  ;[1 1 1] Check If Target In Range
  (cast `/Game/Blueprints/GoblinCharacter` OtherActor)
  (set `self.Player in range` true)
  (`self.Burn`))

(event `Burn`
  (`|ExecutionSequence`
    (:`then_0`
      ;[1 1 1] Player
      (if (`self.Player in range`)
        (`self.Deal damage`)
        (`KismetSystemLibrary.Delay` 0.5 :!label _label)
        (if (`self.Player in range`)
          (`self.Burn`))))
    (:`then_1`
      ;[1 1 1] AI
      (for _array_element (`self.HIttedAI`)
        (`/Game/AI2/EnemyCharacter.Get damage` _array_element 5.0)
        (goto _label)))))

(event `self.Sphere.OnComponentEndOverlap`
  (params (OverlappedComponent :type "PrimitiveComponent Object Reference") (OtherActor :type "Actor Object Reference") (OtherComp :type "PrimitiveComponent Object Reference") (OtherBodyIndex :type Integer))
  ;[1 1 1] Check If Target In Range
  (cast `/Game/Blueprints/GoblinCharacter` OtherActor)
  (set `self.Player in range` false))

(fn `Chase`
  (`self.K2_SetActorRotation` (`KismetMathLibrary.Conv_VectorToRotator` (- (`self.K2_GetActorLocation` (`GameplayStatics.GetPlayerCharacter` 0)) (`self.K2_GetActorLocation`))) true)
  (`ProjectileMovementComponent.SetVelocityInLocalSpace` (`self.ProjectileMovement`) (`KismetMathLibrary.MakeVector` (`self.Speed`)))
  (`self.Burn`))

(fn `UserConstructionScript`
  (`parent.UserConstructionScript`))