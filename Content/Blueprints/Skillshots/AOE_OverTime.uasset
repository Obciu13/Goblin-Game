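; Skillshot area-of-effect actor that deals damage over time to a player in range.
; On BeginPlay it calls ScaleEffect and spawns a scaled fire particle effect at its location.
; Tick runs through a one-second Delay, so roughly once per second it checks PlayerInRange and calls DealDamage, neither of which is defined in these graphs.
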(event `self.ReceiveBeginPlay`
  (`self.Scale_effect`)
  (`GameplayStatics.SpawnEmitterAtLocation` "/Game/StarterContent/Particles/P_Fire.P_Fire" (`self.K2_GetActorLocation`) (struct) (`self.Scale`)))

(event `self.ReceiveTick`
  (params (DeltaSeconds :type "Float (single-precision)"))
  (`parent.ReceiveTick` DeltaSeconds)
  (`KismetSystemLibrary.Delay` 1.0)
  (if (`self.Player in range`)
    (`self.Deal damage`)))

(fn `UserConstructionScript`
  (`parent.UserConstructionScript`))