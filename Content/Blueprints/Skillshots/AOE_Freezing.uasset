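; AOE_Freezing is a skillshot area-of-effect actor that deals damage after a delay and leaves an ice field behind.
; On BeginPlay it calls ScaleEffect, waits for the Delay, spawns a particle burst at double its Scale and calls DealDamage.
; It then spawns an Ice_Field actor at its location, shrunk to a fixed scale, and destroys itself.
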(event `self.ReceiveBeginPlay`
  (bind (_returnvalue_x _returnvalue_y _returnvalue_z) (`KismetMathLibrary.BreakVector` (`self.K2_GetActorLocation`)))
  (`self.Scale_effect`)
  (`KismetSystemLibrary.Delay` (`self.Delay`))
  (`GameplayStatics.SpawnEmitterAtLocation` (`self.Particle System`) (`self.K2_GetActorLocation`) (struct) (* (`self.Scale`) 2))
  (`self.Deal damage`)
  (`|SpawnActorFromClass` "/Game/Blueprints/Skillshots/Ice_Field.Ice_Field_C" (`KismetMathLibrary.MakeTransform` (`KismetMathLibrary.MakeVector` _returnvalue_x _returnvalue_y _returnvalue_z) (struct) (0.8 0.8 0.8)) "Undefined" "OverrideRootScale" null null)
  (`self.K2_DestroyActor`))

(fn `UserConstructionScript`
  (`parent.UserConstructionScript`))