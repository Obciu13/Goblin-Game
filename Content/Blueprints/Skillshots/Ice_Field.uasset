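; Ice field skillshot actor that alters the movement speed of goblin characters inside its sphere, presumably slowing them.
; On spawn it sets a lifetime that scales with player 0's goblin level, then destroys itself.
; Sphere overlap begin and end raise and lower each goblin's Freezed2 counter and call UpdateSpeed, so overlapping fields are counted.
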(event `self.ReceiveBeginPlay`
  (bind _asgoblin_character (cast `/Game/Blueprints/GoblinCharacter` (`GameplayStatics.GetPlayerCharacter` 0)))
  (`KismetSystemLibrary.Delay` (`KismetMathLibrary.Conv_IntToDouble` (+ (* (/ (`/Game/Blueprints/GoblinCharacter.Level` _asgoblin_character) 8) 2) 16)))
  (`self.K2_DestroyActor`))

(event `self.Sphere.OnComponentBeginOverlap`
  (params (OverlappedComponent :type "PrimitiveComponent Object Reference") (OtherActor :type "Actor Object Reference") (OtherComp :type "PrimitiveComponent Object Reference") (OtherBodyIndex :type Integer) (bFromSweep :type Boolean) (SweepResult :type "HitResult Structure (by ref)"))
  (bind _asgoblin_character (cast `/Game/Blueprints/GoblinCharacter` OtherActor))
  (set `/Game/Blueprints/GoblinCharacter.Freezed2` (+ (`/Game/Blueprints/GoblinCharacter.Freezed2` _asgoblin_character) 1) _asgoblin_character)
  (`/Game/Blueprints/GoblinCharacter.UpdateSpeed` _asgoblin_character))

(event `self.Sphere.OnComponentEndOverlap`
  (params (OverlappedComponent :type "PrimitiveComponent Object Reference") (OtherActor :type "Actor Object Reference") (OtherComp :type "PrimitiveComponent Object Reference") (OtherBodyIndex :type Integer))
  (bind _asgoblin_character (cast `/Game/Blueprints/GoblinCharacter` OtherActor))
  (set `/Game/Blueprints/GoblinCharacter.Freezed2` (+ (`/Game/Blueprints/GoblinCharacter.Freezed2` _asgoblin_character) -1) _asgoblin_character)
  (`/Game/Blueprints/GoblinCharacter.UpdateSpeed` _asgoblin_character))

(fn `UserConstructionScript`)