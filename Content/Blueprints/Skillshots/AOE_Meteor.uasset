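; Meteor area-of-effect skillshot actor that deals damage once after a delay, then destroys itself.
; On BeginPlay it calls ScaleEffect with zero and spawns the fire-crack Niagara system below its location, then waits before calling DealDamage.
; ScaleEffect and DealDamage are defined outside this graph.
; The overlap event is disabled, and an older particle emitter spawn is left unconnected.
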(event `self.ReceiveBeginPlay`
  (bind (_returnvalue_x _returnvalue_y _returnvalue_z) (`KismetMathLibrary.BreakVector` (`self.K2_GetActorLocation`)))
  (`self.Scale_effect` (0.0 0.0 0.0))
  (`NiagaraFunctionLibrary.SpawnSystemAtLocation` "/Game/Animations/Fireball_new/NS_Fireball/NiagaraSystems/NS_FireCrack.NS_FireCrack" (`KismetMathLibrary.MakeVector` _returnvalue_x _returnvalue_y (- _returnvalue_z 120.0)))
  (`KismetSystemLibrary.Delay` (`self.Delay`))
  (`self.Deal damage`)
  (`self.K2_DestroyActor`))

(fn `UserConstructionScript`
  (`parent.UserConstructionScript`))