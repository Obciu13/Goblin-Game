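; AOE_Wave is a skillshot Blueprint for a delayed area-of-effect wave attack.
; On BeginPlay it calls ScaleEffect, waits for the Delay time, then spawns its particle system at the actor's location at double its Scale.
; It then calls DealDamage and destroys itself, with neither of those helper functions defined in this graph.
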(event `self.ReceiveBeginPlay`
  (`self.Scale_effect`)
  (`KismetSystemLibrary.Delay` (`self.Delay`))
  (`GameplayStatics.SpawnEmitterAtLocation` (`self.Particle System`) (`self.K2_GetActorLocation`) (struct) (* (`self.Scale`) 2))
  (`self.Deal damage`)
  (`self.K2_DestroyActor`))

(fn `UserConstructionScript`
  (`parent.UserConstructionScript`))