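; Dragons_Breathe is a skillshot actor that lays down a line of fire in a random direction.
; On BeginPlay it picks a random yaw, waits briefly, then starts the Burning event.
; Burning spawns an AOE_Fire actor along the forward vector at a distance scaled by Counter, then re-calls itself after a short delay until the counter limit, so the fire advances outward step by step.
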(event `self.ReceiveBeginPlay`
  (`self.K2_SetActorRotation` (`KismetMathLibrary.MakeRotator` 0.0 0.0 (`KismetMathLibrary.RandomFloatInRange` 0.0 360.0)))
  (`KismetSystemLibrary.Delay` 2.0)
  (`self.Burning`))

(event `Burning`
  ;[1 1 1] Burning
  (`|SpawnActorFromClass` "/Game/Blueprints/Skillshots/AOE_Fire.AOE_Fire_C" (`KismetMathLibrary.MakeTransform` (+ (`self.K2_GetActorLocation`) (* (* (`KismetMathLibrary.GetForwardVector` (`self.K2_GetActorRotation`)) 200.0) (`self.counter`))) (`KismetMathLibrary.MakeRotator` 0.0)) "Undefined" "OverrideRootScale" null null)
  (`KismetSystemLibrary.Delay` 0.2)
  (bind _result (`/Engine/EditorBlueprintResources/StandardMacros.IncrementInt` (`self.counter`))
    (:`  `
      (if (< _result 20)
        (`self.Burning`)))))

(fn `UserConstructionScript`)