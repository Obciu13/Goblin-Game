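; Fire area-of-effect skillshot that repeatedly damages the goblin player and AI in its area, building on a parent class.
; BeginPlay calls ScaleEffect with a zero vector, and a GoblinCharacter overlap sets an in-range flag and starts Burn, cleared when the box overlap ends.
; Burn calls DealDamage for an in-range player and GetDamage on each hit AI, both paths re-triggering it through a shared half-second Delay.
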(event `self.ReceiveBeginPlay`
  ;[1 1 1] Begin Play
  (`self.Scale_effect` (0.0 0.0 0.0)))

(event `Burn`
  ;[1 1 1] Burn
  (`|ExecutionSequence`
    (:`then_0`
      ;;[1 1 1] Player
      (if (`self.Player in range`)
        (`self.Deal damage`)
        (`KismetSystemLibrary.Delay` 0.5 :!label _label)
        (`self.Burn`)))
    (:`then_1`
      ;;[1 1 1] AI
      (for _array_element (`self.HIttedAI`)
        (`/Game/AI2/EnemyCharacter.Get damage` _array_element 1.0)
        (goto _label)))))

(event `self.ReceiveActorBeginOverlap`
  (params (OtherActor :type "Actor Object Reference"))
  ;[1 1 1] Check If Target In Range
  (`parent.ReceiveActorBeginOverlap` OtherActor)
  (cast `/Game/Blueprints/GoblinCharacter` OtherActor)
  (set `self.Player in range` true)
  (`self.Burn`))

(event `self.Box.OnComponentEndOverlap`
  (params (OverlappedComponent :type "PrimitiveComponent Object Reference") (OtherActor :type "Actor Object Reference") (OtherComp :type "PrimitiveComponent Object Reference") (OtherBodyIndex :type Integer))
  ;[1 1 1] Check If Target In Range
  (cast `/Game/Blueprints/GoblinCharacter` OtherActor)
  (set `self.Player in range` false))

(fn `UserConstructionScript`
  (`parent.UserConstructionScript`))