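; Area-of-effect skillshot actor that strikes the goblin player or enemies inside its box after a delay, then destroys itself.
; BeginPlay waits, plays a configurable skeletal animation and particle effect, removes the cylinder mesh, then calls DealDamage.
; Box overlaps track the player flag and an enemy list.
; DealDamage gives the player configurable damage, hitting listed enemies for a fixed amount only when the player is not hit.
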(event `self.ReceiveTick`
  (params (DeltaSeconds :type "Float (single-precision)")))

(event `self.ReceiveBeginPlay`
  ;[1 1 1] Spawning effect
  (`self.Scale_effect` (0.0 0.0 0.0))
  (`KismetSystemLibrary.Delay` (`self.Delay`))
  (`SkinnedMeshComponent.SetSkinnedAssetAndUpdate` (`self.SkeletalMesh`) (`self.Skeletal`) true)
  (`SkeletalMeshComponent.PlayAnimation` (`self.SkeletalMesh`) (`self.SkeletalAnimation`) false)
  (bind _returnvalue (`GameplayStatics.SpawnEmitterAtLocation` (`self.Particle System`) (`self.K2_GetActorLocation`) (struct) (`self.Scale`)))
  (`ActorComponent.K2_DestroyComponent` (`self.Cylinder`))
  (if (`KismetSystemLibrary.IsValid` _returnvalue)
    (`ActorComponent.K2_DestroyComponent` _returnvalue)
    (else
      (`KismetSystemLibrary.Delay` (`self.Animation delay`))))
  (`self.Deal damage`)
  (`KismetSystemLibrary.Delay` 3.0)
  (`self.K2_DestroyActor`))

(event `self.Box.OnComponentBeginOverlap`
  (params (OverlappedComponent :type "PrimitiveComponent Object Reference") (OtherActor :type "Actor Object Reference") (OtherComp :type "PrimitiveComponent Object Reference") (OtherBodyIndex :type Integer) (bFromSweep :type Boolean) (SweepResult :type "HitResult Structure (by ref)"))
  ;[1 1 1] Check if player and terrain in range
  (cast `/Game/Blueprints/GoblinCharacter` OtherActor
    (:`then`
      (set `self.Player in range` true))
    (:`CastFailed`
      (bind _asenemy_character (cast `/Game/AI2/EnemyCharacter` OtherActor))
      (`KismetArrayLibrary.Array_Add` (`self.HIttedAI`) _asenemy_character))))

(event `self.Box.OnComponentEndOverlap`
  (params (OverlappedComponent :type "PrimitiveComponent Object Reference") (OtherActor :type "Actor Object Reference") (OtherComp :type "PrimitiveComponent Object Reference") (OtherBodyIndex :type Integer))
  ;[1 1 1] Check if player left range
  (cast `/Game/Blueprints/GoblinCharacter` OtherActor
    (:`then`
      (set `self.Player in range` false))
    (:`CastFailed`
      (bind _asenemy_character (cast `/Game/AI2/EnemyCharacter` OtherActor))
      (`KismetArrayLibrary.Array_RemoveItem` (`self.HIttedAI`) _asenemy_character))))

(fn `Deal damage`
  (if (`self.Player in range`)
    (bind _asgoblin_character (cast `/Game/Blueprints/GoblinCharacter` (`GameplayStatics.GetPlayerCharacter` 0))
      (:`then`
        (`/Game/Blueprints/GoblinCharacter.Get Damage` _asgoblin_character (`self.Damage`)))
      (:`CastFailed`
        (for _array_element (`self.HIttedAI`) :!label _label
          (`/Game/AI2/EnemyCharacter.Get damage` _array_element 5.0))))
    (else
      (goto _label))))

(fn `Scale_effect`
  (params (scale :type "Vector Structure"))
  (`SceneComponent.K2_SetWorldTransform` (`self.DefaultSceneRoot`) (`KismetMathLibrary.MakeTransform` (.location (`SceneComponent.K2_GetComponentToWorld` (`self.DefaultSceneRoot`))) (.rotation (`SceneComponent.K2_GetComponentToWorld` (`self.DefaultSceneRoot`))) (`self.Scale`)) false false))

(fn `Scale_effect_1`
  (params (scale :type "Vector Structure"))
  (`SceneComponent.K2_SetWorldTransform` (`self.DefaultSceneRoot`) (`KismetMathLibrary.MakeTransform` (.location (`SceneComponent.K2_GetComponentToWorld` (`self.DefaultSceneRoot`))) (.rotation (`SceneComponent.K2_GetComponentToWorld` (`self.DefaultSceneRoot`))) scale) false false))

(fn `Terrain Restriction`)

(fn `UserConstructionScript`)