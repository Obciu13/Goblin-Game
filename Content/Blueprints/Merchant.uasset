(event `self.ReceiveBeginPlay`
  (`KismetSystemLibrary.Delay` 5.0)
  (bind _asgoblin_character (cast `/Game/Blueprints/GoblinCharacter` (`GameplayStatics.GetPlayerCharacter` 0)))
  (if (not (> (`/Game/Blueprints/GoblinCharacter.CaravanSourge Level` _asgoblin_character) 0))
    (`self.K2_DestroyActor`)))

(event `self.Box.OnComponentBeginOverlap`
  (params (OverlappedComponent :type "PrimitiveComponent Object Reference") (OtherActor :type "Actor Object Reference") (OtherComp :type "PrimitiveComponent Object Reference") (OtherBodyIndex :type Integer) (bFromSweep :type Boolean) (SweepResult :type "HitResult Structure (by ref)"))
  (bind _asgoblin_character (cast `/Game/Blueprints/GoblinCharacter` OtherActor))
  (`/Engine/EditorBlueprintResources/StandardMacros.DoOnce` false
    (:`Completed`
      (switch `int` (`KismetMathLibrary.RandomIntegerInRange` 0 1)
        (:`Default`
          (`/Game/Blueprints/GoblinCharacter.Collect Potion` _asgoblin_character "/Game/Blueprints/Potion_HP.Potion_HP_C" :!label _label))
        (:`0`
          (goto _label))
        (:`1`
          (`/Game/Blueprints/GoblinCharacter.Collect Potion` _asgoblin_character "/Game/Blueprints/Potion_Of_Speed.Potion_Of_Speed_C")))
      (`KismetSystemLibrary.PrintString` "Thank you for help"))))

(fn `UserConstructionScript`)