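; Level changer trigger actor that moves the player between StartShopMap and TopDownExampleMap once quests are done.
; On Box overlap it creates a fade widget and plays FadeIn, before checking that the actor is a TopDownCharacter.
; It scans the character's Quests, stopping at the first unchecked one.
; If all pass, it saves variables to the GameInstance and opens the other map; otherwise it shows a NotAllFound widget.
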(event `self.Box.OnComponentBeginOverlap`
  (params (OverlappedComponent :type "PrimitiveComponent Object Reference") (OtherActor :type "Actor Object Reference") (OtherComp :type "PrimitiveComponent Object Reference") (OtherBodyIndex :type Integer) (bFromSweep :type Boolean) (SweepResult :type "HitResult Structure (by ref)"))
  (`|ExecutionSequence`
    (:`then_0`
      (bind _returnvalue (`|CreateWidget` "/Game/UI/DeathScreen/Widget_Fade.Widget_Fade_C" (`GameplayStatics.GetPlayerController` 0)))
      (bind _aswidget_fade (cast `/Game/UI/DeathScreen/Widget_Fade` _returnvalue))
      (set `self.Fade Reference` _aswidget_fade)
      (`UserWidget.AddToViewport` _returnvalue 0))
    (:`then_1`
      (`/Game/UI/DeathScreen/Widget_Fade.Fade In` (`self.Fade Reference`))
      (bind _astop_down_character (cast `/Game/Blueprints/TopDownCharacter` OtherActor))
      (for _array_element (`/Game/Blueprints/TopDownCharacter.Quests` _astop_down_character)
        (if (`/Game/Blueprints/Loot/Item.Check` _array_element)
          (set `self.Quests_done` true)
          (else
            (set `self.Quests_done` false)
            (break))))
      (if (`self.Quests_done`)
        (`/Game/Blueprints/TopDownCharacter.Save variables to GameInstance` _astop_down_character)
        (bind _returnvalue_2 (`GameplayStatics.GetCurrentLevelName` true))
        (if (`KismetStringLibrary.EqualEqual_StrStr` _returnvalue_2 "StartShopMap")
          (`GameplayStatics.OpenLevel` "TopDownExampleMap")
          (else
            (`GameplayStatics.OpenLevel` "StartShopMap")))
        (else
          (bind _returnvalue_3 (`|CreateWidget` "/Game/UI/NotAllFound.NotAllFound_C"))
          (`UserWidget.AddToViewport` _returnvalue_3 0))))))

(fn `UserConstructionScript`)