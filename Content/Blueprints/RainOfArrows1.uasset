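; RainOfArrows1 is an area hazard actor that repeatedly rains AOE_Arrows around its Cylinder component.
; A looping timer plus random delay staggers volleys, with the spawn loop's upper bound scaling with the player GoblinCharacter's Level.
; Arrows spawn at random navmesh-derived XY positions, slightly above the player's height.
; A slower timer destroys the actor once the player is far away in 2D.
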(event `CustomEvent_1`
  (if (> (`KismetMathLibrary.Vector_Distance2D` (`self.K2_GetActorLocation`) (`self.K2_GetActorLocation` (`GameplayStatics.GetPlayerCharacter` 0))) 5000.0)
    (`self.K2_DestroyActor`)))

(event `self.ReceiveBeginPlay`
  (bind _asgoblin_character (cast `/Game/Blueprints/GoblinCharacter` (`GameplayStatics.GetPlayerCharacter` 0)))
  (set `self.Level` (`/Game/Blueprints/GoblinCharacter.Level` _asgoblin_character))
  (`KismetSystemLibrary.K2_SetTimerDelegate` (delegate `CustomEvent_0`) 0.2 true)
  (`KismetSystemLibrary.K2_SetTimerDelegate` (delegate `CustomEvent_1`) 10.0 true))

(event `CustomEvent_0`
  (bind (_returnvalue_x _returnvalue_y _returnvalue_z) (`KismetMathLibrary.BreakVector` (`self.K2_GetActorLocation` (`GameplayStatics.GetPlayerCharacter` 0))))
  (bind _randomlocation (`NavigationSystemV1.K2_GetRandomReachablePointInRadius` (`SceneComponent.K2_GetComponentLocation` (`self.Cylinder`)) 3000.0 null null))
  (`KismetSystemLibrary.Delay` (`KismetMathLibrary.RandomFloat`))
  (for _ (range 12 (+ (+ 8 (/ (`self.Level`) 2)) 1))
    (`|SpawnActorFromClass` "/Game/Blueprints/Skillshots/AOE_Arrows.AOE_Arrows_C" (`KismetMathLibrary.MakeTransform` (`KismetMathLibrary.MakeVector` (.x _randomlocation) (.y _randomlocation) (+ _returnvalue_z 50.0))) "Undefined" "OverrideRootScale" null (1.0 1.0 1.0) null)))

(fn `UserConstructionScript`)