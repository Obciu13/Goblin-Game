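; Balist is a ballista trap actor that fires at the GoblinCharacter while it is inside the Hitbox.
; Entering the Hitbox starts an Aim cycle, which shows a stretched indicator, waits briefly, then spawns a short-lived projectile from the Projectile component's transform.
; After a cooldown, Aim calls itself again while the goblin remains in range, with an IsAiming flag blocking overlapping cycles.
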(event `Aim`
  (bind (_returnvalue_location _returnvalue_rotation) (`KismetMathLibrary.BreakTransform` (`SceneComponent.K2_GetComponentToWorld` (`self.StaticMesh11`))))
  ;[1 1 1] Aim
  (set `self.IsAiming` true)
  (bind _returnvalue (`|SpawnActorFromClass` "/Game/Blueprints/Balist_Indicator.Balist_Indicator_C" (`KismetMathLibrary.MakeTransform` _returnvalue_location _returnvalue_rotation (20.0 1.5 0.05)) "Undefined" "OverrideRootScale" null null))
  (`GameplayStatics.PlaySound2D` "/Game/Sounds/Effects/New_Sounds/balista_draw.balista_draw" 1.0 1.0 0.0 null null)
  (`KismetSystemLibrary.Delay` 0.5)
  (`self.K2_DestroyActor` _returnvalue)
  (`self.Shoot`)
  (`KismetSystemLibrary.Delay` 3.0)
  (set `self.IsAiming` false)
  (if (`self.Player in range`)
    (`self.Aim`)))

(event `self.Hitbox.OnComponentBeginOverlap`
  (params (OverlappedComponent :type "PrimitiveComponent Object Reference") (OtherActor :type "Actor Object Reference") (OtherComp :type "PrimitiveComponent Object Reference") (OtherBodyIndex :type Integer) (bFromSweep :type Boolean) (SweepResult :type "HitResult Structure (by ref)"))
  ;[1 1 1] Check If Player In Range
  (cast `/Game/Blueprints/GoblinCharacter` OtherActor)
  (set `self.Player in range` true)
  (if (not (`self.IsAiming`))
    (`self.Aim`)))

(event `Shoot`
  ;[1 1 1] Shoot
  (bind _returnvalue (`|SpawnActorFromClass` "/Game/Blueprints/Balist_Projectile.Balist_Projectile_C" (`SceneComponent.K2_GetComponentToWorld` (`self.Projectile`)) "AlwaysSpawn" "OverrideRootScale" null null))
  (`GameplayStatics.PlaySound2D` "/Game/Sounds/Effects/New_Sounds/ArcherShoot.ArcherShoot" 1.0 1.0 0.0 null null)
  (`KismetSystemLibrary.Delay` 0.8)
  (`self.K2_DestroyActor` _returnvalue))

(event `self.Hitbox.OnComponentEndOverlap`
  (params (OverlappedComponent :type "PrimitiveComponent Object Reference") (OtherActor :type "Actor Object Reference") (OtherComp :type "PrimitiveComponent Object Reference") (OtherBodyIndex :type Integer))
  ;[1 1 1] Check If Player In Range
  (cast `/Game/Blueprints/GoblinCharacter` OtherActor)
  (set `self.Player in range` false))

(fn `UserConstructionScript`)