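; MyGameInstance is the GameInstance that holds player progress across levels: gold, max health, drop chances, upgrade levels, potion class, tutorial flag and game phase.
; Its only graph logic is a Reset event that restores every one of these values to its starting default, clearing upgrades such as Gold Sniffing, Tenacity, Caravan Scourge, Corpse Robber and Alchemist.
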(event `Reset`
  (set `self.Gold` 0)
  (set `self.MaxHp` 3.0)
  (set `self.GoldSniffingLevel` 0)
  (set `self.Gold_Drop_Chance` 0.2)
  (set `self.Potion_Drop_Chance` 0.05)
  (set `self.Tenacity Level` 0)
  (set `self.PotionClass` null)
  (set `self.CaravanScourge Level` 0)
  (set `self.Durability Level` 0)
  (set `self.CorpseRobberGold Level` 0)
  (set `self.CorpseRobberPotion Level` 0)
  (set `self.MagicGadgetMaster Level` 0)
  (set `self.Alchemist_Level` 0)
  (set `self.Tutorial` false)
  (set `self.Gold_Given` 0)
  (set `self.Game Phase` ""))