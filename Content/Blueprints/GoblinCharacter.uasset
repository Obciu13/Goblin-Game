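; Player goblin Character that handles movement, health, gold, loot pop-ups, slows, pausing, and win or death flow.
; Stats and potion class persist between levels through MyGameInstance; death cuts gold before saving and returns to StartShopMap.
; Damage triggers temporary invulnerability with recursive red material blinking.
; Space performs a teleport dash on a delay-counted cooldown, and E uses the potion held in a ChildActor component.
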(event `Get Damage`
  (params (Damage :type "Float (double-precision)"))
  ;[1 1 1] Get Damage
  (if (not (`self.Resistance`))
    (bind _output_get (set `self.HP` (- (`self.HP`) Damage)))
    (if (<= _output_get 0.0)
      (`self.Event Death`)
      (else
        (set `self.Resistance` true)
        (`self.Blinking after dmg`)))))

(event `self.ReceiveBeginPlay`
  ;[1 1 1] Event BeginPlay
  (`|ExecutionSequence`
    (:`then_0`
      (bind _returnvalue (`|CreateWidget` "/Game/UI/DeathScreen/Widget_Fade.Widget_Fade_C" (`GameplayStatics.GetPlayerController` 0)))
      (bind _aswidget_fade (cast `/Game/UI/DeathScreen/Widget_Fade` _returnvalue))
      (set `self.Fade Reference` _aswidget_fade)
      (`UserWidget.AddToViewport` _returnvalue 0))
    (:`then_1`
      (`/Game/UI/DeathScreen/Widget_Fade.Fade In` (`self.Fade Reference`))
      (bind _returnvalue_2 (`|CreateWidget` "/Game/UI/Hud.Hud_C"))
      (`UserWidget.AddToViewport` _returnvalue_2 0)
      (`self.Load from GameInstance`))))

(event `Event Death`
  ;[1 1 1] Event Death
  (`self.DisableInput` (`GameplayStatics.GetPlayerCharacter` 0) (`GameplayStatics.GetPlayerController` 0))
  (`/Game/UI/DeathScreen/Widget_Fade.Fade Off` (`self.Fade Reference`))
  (`KismetSystemLibrary.Delay` 1.0)
  (bind _returnvalue (`|CreateWidget` "/Game/UI/DeathScreen/DeathScreen.DeathScreen_C"))
  (`UserWidget.AddToViewport` _returnvalue 0)
  (set `self.Gold` (`KismetMathLibrary.FTrunc` (* (`self.Gold`) 0.8)))
  (`self.Save variables to GameInstance`)
  (`KismetSystemLibrary.Delay` 1.0)
  (`GameplayStatics.OpenLevel` "StartShopMap"))

(event `InputAxis|MoveForward`
  (params (AxisValue :type "Float (single-precision)"))
  ;[1 1 1] Character Controll
  (`self.AddMovementInput` (90.0 0.0 0.0) AxisValue))

(event `InputAxis|MoveRight`
  (params (AxisValue :type "Float (single-precision)"))
  ;[1 1 1] Character Controll
  (`self.AddMovementInput` (0.0 90.0 0.0) AxisValue))

(event `Get Gold`
  (params (`Income gold` :type Integer))
  ;[1 1 1] Get Gold Event
  (set `self.Income Gold` `Income gold`)
  (set `self.Gold` (+ (`self.Gold`) (`self.Income Gold`)))
  (bind _returnvalue (`|CreateWidget` "/Game/UI/GoldPopUp.GoldPopUp_C"))
  (`UserWidget.AddToViewport` _returnvalue 0))

(event `WonLevel`
  ;[1 1 1] Event Won level
  (`self.Save variables to GameInstance`)
  (`GameplayStatics.SetGamePaused` true)
  (bind _returnvalue (`|CreateWidget` "/Game/UI/BattleSurvived.BattleSurvived_C" (`GameplayStatics.GetPlayerController` 0)))
  (`UserWidget.AddToViewport` _returnvalue 0))

(event `Key|SpaceBar`
  (params (Key :type "Key Structure"))
  (bind _returnvalue (`GameplayStatics.GetPlayerCharacter` 0))
  ;[1 1 1] Dash
  (:`Pressed`
    (if (== (`self.Dashcounter`) (`self.Dashcooldown`))
      (`self.K2_TeleportTo` (+ (`self.K2_GetActorLocation` _returnvalue) (* (`self.GetActorForwardVector` _returnvalue) (`self.DashRange`))) (`self.K2_GetActorRotation` _returnvalue))
      (set `self.Dashcounter` 0.0)
      (if (< (`self.Dashcounter`) (`self.Dashcooldown`)) :!label _label
        (`KismetSystemLibrary.Delay` 1.0)
        (`/Engine/EditorBlueprintResources/StandardMacros.IncrementFloat` (`self.Dashcounter`)
          (:`  `
            (goto _label)))))))

(event `Save variables to GameInstance`
  (bind _returnvalue (`GameplayStatics.GetObjectClass` (`ChildActorComponent.ChildActor` (`self.Potion'`))))
  ;[1 1 1] Saving chosen variables to game instance (to save them between levels)
  (bind _asmy_game_instance (cast `/Game/Blueprints/MyGameInstance` (`GameplayStatics.GetGameInstance`)))
  (set `/Game/Blueprints/MyGameInstance.Gold` (`self.Gold`) _asmy_game_instance)
  (set `/Game/Blueprints/MyGameInstance.MaxHp` (`self.MaxHP`) _asmy_game_instance)
  (set `/Game/Blueprints/MyGameInstance.HarvestingSpeedUp` (`self.HarvestingSpeedUp`) _asmy_game_instance)
  (set `/Game/Blueprints/MyGameInstance.Gold_Drop_Chance` (`self.GoldDropChance`) _asmy_game_instance)
  (set `/Game/Blueprints/MyGameInstance.Potion_Drop_Chance` (`self.PotionDropChance`) _asmy_game_instance)
  (set `/Game/Blueprints/MyGameInstance.Tenacity` (`self.Tenacity`) _asmy_game_instance)
  (set `/Game/Blueprints/MyGameInstance.PotionClass` _returnvalue _asmy_game_instance)
  (`KismetSystemLibrary.PrintString` (`KismetSystemLibrary.GetClassDisplayName` _returnvalue)))

(event `Load from GameInstance`
  ;[1 1 1] Load variables from GameInstance
  (bind _asmy_game_instance (cast `/Game/Blueprints/MyGameInstance` (`GameplayStatics.GetGameInstance`)))
  (set `self.Gold` (`/Game/Blueprints/MyGameInstance.Gold` _asmy_game_instance))
  (bind _output_get (set `self.MaxHP` (`/Game/Blueprints/MyGameInstance.MaxHp` _asmy_game_instance)))
  (set `self.HP` _output_get)
  (set `self.HarvestingSpeedUp` (`/Game/Blueprints/MyGameInstance.HarvestingSpeedUp` _asmy_game_instance))
  (set `self.GoldDropChance` (`/Game/Blueprints/MyGameInstance.Gold_Drop_Chance` _asmy_game_instance))
  (set `self.PotionDropChance` (`/Game/Blueprints/MyGameInstance.Potion_Drop_Chance` _asmy_game_instance))
  (set `self.Tenacity` (`/Game/Blueprints/MyGameInstance.Tenacity` _asmy_game_instance))
  (bind _potionclass (`/Game/Blueprints/MyGameInstance.PotionClass` _asmy_game_instance))
  (`ChildActorComponent.SetChildActorClass` (`self.Potion'`) _potionclass)
  (`KismetSystemLibrary.PrintString` (`KismetSystemLibrary.GetClassDisplayName` _potionclass)))

(event `InputAction|PauseEvent`
  (params (Key :type "Key Structure"))
  (bind _returnvalue (`GameplayStatics.GetPlayerController` 0))
  ;[1 1 1] Pause
  (:`Pressed`
    (`GameplayStatics.SetGamePaused` true)
    (bind _returnvalue_2 (`|CreateWidget` "/Game/UI/Pause.Pause_C"))
    (`UserWidget.AddToViewport` _returnvalue_2 0)
    (`WidgetBlueprintLibrary.SetInputMode_UIOnlyEx` _returnvalue _returnvalue_2)
    (set `PlayerController.bShowMouseCursor` true _returnvalue)))

(event `Get reward`
  (params (Reward :type "/Game/Blueprints/Loot/Item Object Reference"))
  ;[1 1 1] Get Reward (Items loot system)
  (set `/Game/Blueprints/Loot/Item.Check` true Reward)
  (set `self.Reward Name` (`/Game/Blueprints/Loot/Item.Name` Reward))
  (bind _returnvalue (`|CreateWidget` "/Game/UI/FindItemPopUp.FindItemPopUp_C"))
  (`UserWidget.AddToViewport` _returnvalue 0))

(event `Get Slowed`
  (params (Slow :type "Float (double-precision)"))
  (bind _charactermovement (`self.CharacterMovement`))
  ;[1 1 1] Get Slowed
  (set `CharacterMovementComponent.MaxWalkSpeed` (* (+ Slow (`self.Tenacity`)) (`CharacterMovementComponent.MaxWalkSpeed` _charactermovement)) _charactermovement))

(event `Blinking after dmg`
  ;[1 1 1] Red blinking
  (`self.Change Color` true)
  (`KismetSystemLibrary.Delay` 0.1)
  (`self.Change Color` false)
  (`KismetSystemLibrary.Delay` 0.1)
  (bind _result (`/Engine/EditorBlueprintResources/StandardMacros.IncrementInt` (`self.Blinking counter`))
    (:`  `
      (if (< _result 10)
        (`self.Blinking after dmg`)
        (else
          (set `self.Resistance` false)
          (set `self.Blinking counter` 0))))))

(event `Return to base speed`
  ;[1 1 1] Return to base speed
  (set `CharacterMovementComponent.MaxWalkSpeed` (`self.Base speed`) (`self.CharacterMovement`)))

(event `Collect Potion`
  (params (Class :type "Actor Class Reference"))
  ;[1 1 1] Collect Potion
  (`ChildActorComponent.SetChildActorClass` (`self.Potion'`) Class))

(event `Key|E`
  (params (Key :type "Key Structure"))
  ;[1 1 1] E input
  (:`Pressed`
    (`self.Use Potion`)))

(event `Use Potion`
  (bind _childactor (`ChildActorComponent.ChildActor` (`self.Potion'`)))
  ;[1 1 1] Use Potion
  (if (`KismetSystemLibrary.IsValid` _childactor)
    (bind _aspotion__eq (cast `/Game/Blueprints/Potion-EQ` _childactor))
    (`/Game/Blueprints/Potion-EQ.Use` _aspotion__eq)
    (else
      (`KismetSystemLibrary.PrintString` "Nie masz nic do picia"))))

(fn `Change Color`
  (params (GetDmg :type Boolean))
  (locals (NewLocalVar_0 :type Boolean))
  (if GetDmg
    (for (_ _array_index) (`self.Materials`)
      (`PrimitiveComponent.SetMaterial` (`self.Mesh`) _array_index "/Game/Textures/RedOnHit.RedOnHit"))
    (else
      (for (_array_element _array_index_2) (`self.Materials`)
        (`PrimitiveComponent.SetMaterial` (`self.Mesh`) _array_index_2 _array_element)))))

(fn `UserConstructionScript`)