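; Shaman enemy that casts spells at the player while a GoblinCharacter is inside its sphere trigger.
; CastSpell randomly picks a projectile volley, a freezing AOE near the player or a tornado at itself, then repeats after a delay while in range.
; The volley re-calls itself with a counter, aiming each shot at the player's current location.
; Pull and Wave spells are defined but never called here.
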(event `self.Sphere.OnComponentBeginOverlap`
  (params (OverlappedComponent :type "PrimitiveComponent Object Reference") (OtherActor :type "Actor Object Reference") (OtherComp :type "PrimitiveComponent Object Reference") (OtherBodyIndex :type Integer) (bFromSweep :type Boolean) (SweepResult :type "HitResult Structure (by ref)"))
  ;[1 1 1] Overlap
  (cast `/Game/Blueprints/GoblinCharacter` OtherActor)
  (set `self.Player in Range` true)
  (`self.Cast Spell`))

(event `self.Sphere.OnComponentEndOverlap`
  (params (OverlappedComponent :type "PrimitiveComponent Object Reference") (OtherActor :type "Actor Object Reference") (OtherComp :type "PrimitiveComponent Object Reference") (OtherBodyIndex :type Integer))
  ;[1 1 1] Overlap
  (cast `/Game/Blueprints/GoblinCharacter` OtherActor)
  (set `self.Player in Range` false))

(event `Cast Spell`
  ;[1 1 1] Cast Spell
  (if (`self.Player in Range`)
    (switch `int` (`KismetMathLibrary.RandomIntegerInRange` 0 2)
      (:`0`
        (`self.Projectiles`)
        (`KismetSystemLibrary.Delay` 10.0))
      (:`1`
        (`self.Freezing`)
        (`KismetSystemLibrary.Delay` 10.0))
      (:`2`
        (`self.Tornado`)
        (`KismetSystemLibrary.Delay` 10.0)))
    (set `self.Counter` 0)
    (`self.Cast Spell`)))

(event `Freezing`
  (bind _returnvalue (`self.K2_GetActorLocation` (`GameplayStatics.GetPlayerCharacter` 0)))
  (bind _randomlocation (`NavigationSystemV1.K2_GetRandomReachablePointInRadius` _returnvalue 100.0 null null))
  ;[1 1 1] Freezing
  (`/Engine/EditorBlueprintResources/StandardMacros.IncrementInt` (`self.Counter`)
    (:`  `
      (`KismetSystemLibrary.Delay` 0.5)
      (`SkeletalMeshComponent.PlayAnimation` (`self.SkeletalMesh`) "/Game/OrcModel/Orc_ShamanModel/Orc1shaman_Anim_OrcShaman_Small_Fireball.Orc1shaman_Anim_OrcShaman_Small_Fireball" false)
      (`|SpawnActorFromClass` "/Game/Blueprints/Skillshots/AOE_Freezing.AOE_Freezing_C" (`KismetMathLibrary.Conv_VectorToTransform` (`KismetMathLibrary.MakeVector` (.x _randomlocation) (.y _randomlocation) (+ (.z _returnvalue) 50.0))) "Undefined" "OverrideRootScale" null null))))

(event `Projectiles`
  (bind (_returnvalue_x _returnvalue_y _returnvalue_z) (`KismetMathLibrary.BreakVector` (`self.K2_GetActorLocation` self)))
  (bind _returnvalue (`self.GetTransform` self))
  (bind (_returnvalue_x_2 _returnvalue_y_2 _returnvalue_z_2) (`KismetMathLibrary.BreakVector` (* (`KismetMathLibrary.GetDirectionUnitVector` (`KismetMathLibrary.MakeVector` _returnvalue_x _returnvalue_y (+ _returnvalue_z 200.0)) (`self.K2_GetActorLocation` (`GameplayStatics.GetPlayerCharacter` 0))) 1200)))
  ;[1 1 1] Projectiles
  (`KismetSystemLibrary.Delay` 1.0)
  (`SkeletalMeshComponent.PlayAnimation` (`self.SkeletalMesh`) "/Game/OrcModel/Orc_ShamanModel/Orc1shaman_Anim_OrcShaman_Small_Fireball.Orc1shaman_Anim_OrcShaman_Small_Fireball" false)
  (bind _returnvalue_2 (`|SpawnActorFromClass` "/Game/Blueprints/Skillshots/Magic_Projectile.Magic_Projectile_C" (`KismetMathLibrary.MakeTransform` (`KismetMathLibrary.MakeVector` (.x (.location _returnvalue)) (.y (.location _returnvalue)) (+ (.z (.location _returnvalue)) 200.0)) (.rotation _returnvalue) (.scale _returnvalue)) "Undefined" "OverrideRootScale" null null))
  (set `MovementComponent.Velocity` (`KismetMathLibrary.MakeVector` _returnvalue_x_2 _returnvalue_y_2 _returnvalue_z_2) (`/Game/Blueprints/Skillshots/Magic_Projectile.ProjectileMovement` _returnvalue_2))
  (bind _result (`/Engine/EditorBlueprintResources/StandardMacros.IncrementInt` (`self.Counter`))
    (:`  `
      (if (< _result 6)
        (`KismetSystemLibrary.Delay` 0.5)
        (`self.Projectiles`)))))

(event `Pull`
  ;[1 1 1] Pull
  (`|SpawnActorFromClass` "/Game/Blueprints/Skillshots/AOE_Pull.AOE_Pull_C" (`KismetMathLibrary.MakeTransform` (`KismetMathLibrary.MakeVector` (.x (.location (`self.GetTransform`))) (.y (.location (`self.GetTransform`))) (+ (.z (`self.K2_GetActorLocation` (`GameplayStatics.GetPlayerCharacter` 0))) 50.0))) "Undefined" "OverrideRootScale" null null))

(event `Tornado`
  ;[1 1 1] Tornado
  (`SkeletalMeshComponent.PlayAnimation` (`self.SkeletalMesh`) "/Game/OrcModel/Orc_ShamanModel/Orc1shaman_Anim_OrcShaman_Pull.Orc1shaman_Anim_OrcShaman_Pull" false)
  (`|SpawnActorFromClass` "/Game/Blueprints/Skillshots/AOE_Tornado.AOE_Tornado_C" (`self.GetTransform`) "AlwaysSpawn" "OverrideRootScale" null null)
  (`KismetSystemLibrary.Delay` 10.0))

(event `Wave`
  (bind _returnvalue (`self.K2_GetActorLocation`))
  (bind _returnvalue_2 (`KismetMathLibrary.GetDirectionUnitVector` _returnvalue (`self.Target location`)))
  ;[1 1 1] Wave
  (`/Engine/EditorBlueprintResources/StandardMacros.IncrementInt` (`self.Counter`)
    (:`  `
      (`|SpawnActorFromClass` "/Game/Blueprints/Skillshots/AOE_Wave.AOE_Wave_C" (`KismetMathLibrary.MakeTransform` (`KismetMathLibrary.MakeVector` (.x (+ (* (* _returnvalue_2 300) (`self.Counter`)) _returnvalue)) (.y (+ (* (* _returnvalue_2 300) (`self.Counter`)) _returnvalue)) (+ (.z (`self.K2_GetActorLocation` (`GameplayStatics.GetPlayerCharacter` 0))) 50.0)) (`KismetMathLibrary.Quat_Rotator` (`KismetMathLibrary.Conv_VectorToQuaternion` _returnvalue_2))) "Undefined" "OverrideRootScale" null null)
      (`KismetSystemLibrary.Delay` 0.2)
      (if (<= (`self.Counter`) 5)
        (`SkeletalMeshComponent.PlayAnimation` (`self.SkeletalMesh`) "/Game/OrcModel/Orc_ShamanModel/Orc1shaman_Anim_OrcShaman_Small_Fireball.Orc1shaman_Anim_OrcShaman_Small_Fireball" false)
        (`self.Wave`)))))

(fn `UserConstructionScript`)