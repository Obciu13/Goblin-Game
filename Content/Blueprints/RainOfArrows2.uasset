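; Rain of Arrows actor that spawns an area volley of AOE_Arrows actors in three staggered waves.
; On BeginPlay it sets a random yaw to vary the pattern, then collects static mesh components tagged Phase1, Phase2 and Phase3.
; The tagged meshes act as spawn markers, each supplying the world transform for one arrow actor, with a short delay between waves.
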(event `self.ReceiveBeginPlay`
  (`self.K2_SetActorRotation` (`KismetMathLibrary.MakeRotator` 0.0 0.0 (`KismetMathLibrary.RandomFloatInRange` 0.0 360.0)))
  (bind _output_get (set `self.Phase1` (`self.GetComponentsByTag` "/Script/Engine.StaticMeshComponent" "Phase1")))
  (set `self.Phase2` (`self.GetComponentsByTag` "/Script/Engine.StaticMeshComponent" "Phase2"))
  (set `self.Phase3` (`self.GetComponentsByTag` "/Script/Engine.StaticMeshComponent" "Phase3"))
  (for _array_element _output_get
    (`|SpawnActorFromClass` "/Game/Blueprints/Skillshots/AOE_Arrows.AOE_Arrows_C" (`SceneComponent.K2_GetComponentToWorld` _array_element) "Undefined" "OverrideRootScale" null (1.0 1.0 1.0) null))
  (`KismetSystemLibrary.Delay` 0.2)
  (for _array_element_2 (`self.Phase2`)
    (`|SpawnActorFromClass` "/Game/Blueprints/Skillshots/AOE_Arrows.AOE_Arrows_C" (`SceneComponent.K2_GetComponentToWorld` _array_element_2) "Undefined" "OverrideRootScale" null (1.0 1.0 1.0) null))
  (`KismetSystemLibrary.Delay` 0.2)
  (for _array_element_3 (`self.Phase3`)
    (`|SpawnActorFromClass` "/Game/Blueprints/Skillshots/AOE_Arrows.AOE_Arrows_C" (`SceneComponent.K2_GetComponentToWorld` _array_element_3) "Undefined" "OverrideRootScale" null (1.0 1.0 1.0) null)))

(fn `UserConstructionScript`)