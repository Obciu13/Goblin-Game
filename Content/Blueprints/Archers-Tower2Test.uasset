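; Archer tower that aims at the player's goblin while it is inside the Sphere trigger, then shoots after a countdown.
; A looping timer handles cooldown, turns the archer toward the player and aims a red laser beam.
; A line trace toward the player decides who takes damage, goblin or intercepting enemy.
; An on-screen aim widget shows while the trace hits the player; losing that hit resets the aim and starts cooldown.
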(event `self.ReceiveBeginPlay`
  (`SceneComponent.K2_SetWorldTransform` (`self.Bow`) (`SceneComponent.GetSocketTransform` (`self.SkeletalMesh`) "WeaponHold" "RTS_World") false false)
  (`SceneComponent.K2_AttachToComponent` (`self.Bow`) (`self.SkeletalMesh`) "WeaponHold" "SnapToTarget" "SnapToTarget" "SnapToTarget" true))

(event `self.Sphere.OnComponentBeginOverlap`
  (params (OverlappedComponent :type "PrimitiveComponent Object Reference") (OtherActor :type "Actor Object Reference") (OtherComp :type "PrimitiveComponent Object Reference") (OtherBodyIndex :type Integer) (bFromSweep :type Boolean) (SweepResult :type "HitResult Structure (by ref)"))
  ;[1 1 1] Overlap Managment
  (cast `/Game/Blueprints/GoblinCharacter` OtherActor)
  (set `self.Player in Range` true)
  (bind _returnvalue (`KismetSystemLibrary.K2_SetTimerDelegate` (delegate `Custom Tick`) 0.01 true)))

(event `self.Sphere.OnComponentEndOverlap`
  (params (OverlappedComponent :type "PrimitiveComponent Object Reference") (OtherActor :type "Actor Object Reference") (OtherComp :type "PrimitiveComponent Object Reference") (OtherBodyIndex :type Integer))
  ;[1 1 1] Overlap Managment
  (cast `/Game/Blueprints/GoblinCharacter` OtherActor)
  (set `self.Player in Range` false)
  (set `self.Aim_Timer` 5.0)
  (`self.ResetAimIndicator`)
  (`KismetSystemLibrary.K2_PauseTimerHandle` (stale `self.Sphere.OnComponentBeginOverlap` _returnvalue)))

(event `Custom Tick`
  (bind (_returnvalue_roll _returnvalue_pitch _returnvalue_yaw) (`KismetMathLibrary.BreakRotator` (`KismetMathLibrary.FindLookAtRotation` (`SceneComponent.K2_GetComponentLocation` (`self.SkeletalMesh`)) (`self.K2_GetActorLocation` (`GameplayStatics.GetPlayerCharacter` 0)))))
  (if (`self.Player in Range`)
    ;[1 1 1] Cooldown Managment
    (if (> (`self.Cooldown`) 0.0)
      (`KismetSystemLibrary.Delay` 1.0)
      (`/Engine/EditorBlueprintResources/StandardMacros.DecrementFloat` (`self.Cooldown`))
      (else
        (`|ExecutionSequence`
          (:`then_0`
            (`SceneComponent.K2_SetWorldRotation` (`self.SkeletalMesh`) (`KismetMathLibrary.MakeRotator` 0.0 0.0 (- _returnvalue_yaw 90.0)) false false)
            ;[1 1 1] Update Indicator Position
            (bind _outhit (`KismetSystemLibrary.LineTraceSingleForObjects` :`Start` (`SceneComponent.K2_GetComponentLocation` (`self.Archer`)) :`End` (`self.K2_GetActorLocation` (`GameplayStatics.GetPlayerCharacter` 0)) :`ObjectTypes` (`|MakeArray` "ObjectTypeQuery1" "ObjectTypeQuery3" "ObjectTypeQuery2" :!type "EObjectTypeQuery Enum") :`TraceColor` (`self.Trace color`) :`TraceHitColor` (`self.Trace hit color`) :`DrawTime` 0.1))
            (`self.UpdateLaser` 0.0)
            (`|ExecutionSequence`
              (:`then_0`
                ;[1 1 1] Check Timer and Target
                (`KismetSystemLibrary.Delay` 1.0)
                (bind _result (`/Engine/EditorBlueprintResources/StandardMacros.DecrementFloat` (`self.Aim_Timer`))
                  (:`  `
                    (if (<= _result 0.0)
                      (`SkeletalMeshComponent.PlayAnimation` (`self.SkeletalMesh`) "/Game/Animations/Bowman/Bowmna_idle.Bowmna_idle" false)
                      (bind (_bblockinghit _binitialoverlap _time _distance _location _impactpoint _normal _impactnormal _physmat _hitactor) (`GameplayStatics.BreakHitResult` _outhit))
                      ;[1 1 1] Deal Damage
                      (bind _asgoblin_character (cast `/Game/Blueprints/GoblinCharacter` _hitactor)
                        (:`then`
                          (`/Game/Blueprints/GoblinCharacter.Get Damage` _asgoblin_character 1.0))
                        (:`CastFailed`
                          (bind _asenemy_character (cast `/Game/AI2/EnemyCharacter` _hitactor)
                            (:`then`
                              (`/Game/AI2/EnemyCharacter.Get damage` _asenemy_character 5.0))
                            (:`CastFailed`
                              _))))
                      ;[1 1 1] Reset Indicator and Timer
                      (set `self.Aim_Timer` 5.0)
                      (set `self.Cooldown` 5.0)
                      (`ActorComponent.K2_DestroyComponent` (`self.Laser`))
                      (`self.Reset laser`)
                      (`self.ResetAimIndicator`)))))
              (:`then_1`
                ;[1 1 1] Aim Indicator Managment
                (if (`self.ActorHasTag` _hitactor "Player")
                  (`/Engine/EditorBlueprintResources/StandardMacros.DoOnce` false :!label _label
                    (:`Completed`
                      (bind _returnvalue (`|CreateWidget` "/Game/UI/AimIndicator.AimIndicator_C"))
                      (`UserWidget.AddToViewport` _returnvalue 0)
                      (set `self.AimIndicator` _returnvalue)))
                  (else
                    (`self.ResetAimIndicator`)
                    (set `self.Aim_Timer` 5.0)
                    (set `self.Cooldown` 5.0)
                    (`ActorComponent.K2_DestroyComponent` (`self.Laser`))
                    (`self.Reset laser`)
                    (`self.ResetAimIndicator`))))))
          (:`then_1`
            ;[1 1 1] Spawn Indicator
            (`/Engine/EditorBlueprintResources/StandardMacros.DoOnce` false :!label _label_2
              (:`Completed`
                (bind _returnvalue_2 (`GameplayStatics.SpawnEmitterAttached` "/Game/Geometry/Meshes/Effects/LaserBeamRED_Particle.LaserBeamRED_Particle" (`self.Archer`) "None" (0.0 0.0 0.0) (struct) (10.0 10.0 10.0) "KeepRelativeOffset" true "AutoRelease"))
                (set `self.Laser` _returnvalue_2)))))))))

(event `Reset Indicator`
  ;[1 1 1] Aim Indicator Managment
  (goto _label :!via `Reset`))

(event `Reset laser`
  (goto _label_2 :!via `Reset`))

(fn `IsPlayerInRange`
  (returns (InRange :type Boolean))
  (return (`KismetMathLibrary.InRange_FloatFloat` (`KismetMathLibrary.Vector_Distance` (`self.K2_GetActorLocation` self) (`self.K2_GetActorLocation` (`GameplayStatics.GetPlayerCharacter` 0))) (`self.Min_Range`) (`self.Max_Range`))))

(fn `ResetAimIndicator`
  (if (`KismetSystemLibrary.IsValid` (`self.AimIndicator`))
    (`Widget.RemoveFromParent` (`self.AimIndicator`))
    (`self.Reset Indicator`)))

(fn `UpdateLaser`
  (params (Aim_timer :type "Float (double-precision)"))
  (if (`KismetSystemLibrary.IsValid` (`self.Laser`))
    (`SceneComponent.K2_SetWorldRotation` (`self.Laser`) (`KismetMathLibrary.Conv_VectorToRotator` (- (`self.K2_GetActorLocation` (`GameplayStatics.GetPlayerCharacter` 0)) (`SceneComponent.K2_GetComponentLocation` (`self.Archer`)))) false false)))

(fn `UserConstructionScript`)