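; Giant Orc NPC that opens a dialog when the GoblinCharacter overlaps its Box component.
; During the TutorialPart2 phase it shows the first-meeting dialog, advances the goblin's GamePhase to Game and spawns a Golden_Circle at a hard-coded location.
; In any other phase it shows the common dialog.
; Both dialogs pause the game and switch input to UI only with the mouse cursor visible.
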(event `self.Box.OnComponentBeginOverlap`
  (params (OverlappedComponent :type "PrimitiveComponent Object Reference") (OtherActor :type "Actor Object Reference") (OtherComp :type "PrimitiveComponent Object Reference") (OtherBodyIndex :type Integer) (bFromSweep :type Boolean) (SweepResult :type "HitResult Structure (by ref)"))
  (bind _returnvalue (`GameplayStatics.GetPlayerController` 0))
  (bind _returnvalue_2 (`GameplayStatics.GetPlayerController` 0))
  (bind _asgoblin_character (cast `/Game/Blueprints/GoblinCharacter` OtherActor))
  (bind _output_get (set `self.As Goblin Character` _asgoblin_character))
  (if (`KismetStringLibrary.EqualEqual_StrStr` (`/Game/Blueprints/GoblinCharacter.GamePhase` _output_get) "TutorialPart2")
    ;[1 1 1] First Dialog
    (bind _returnvalue_3 (`|CreateWidget` "/Game/UI/GiantOrc/GiantOrcFirstDialog.GiantOrcFirstDialog_C"))
    (`UserWidget.AddToViewport` _returnvalue_3 0)
    (`WidgetBlueprintLibrary.SetInputMode_UIOnlyEx` _returnvalue_2 _returnvalue_3)
    (set `PlayerController.bShowMouseCursor` true _returnvalue_2)
    (`GameplayStatics.SetGamePaused` true)
    (set `/Game/Blueprints/GoblinCharacter.GamePhase` "Game" (`self.As Goblin Character`))
    (`|SpawnActorFromClass` "/Game/Blueprints/Golden_Circle.Golden_Circle_C" (`KismetMathLibrary.MakeTransform` (-4507.0 -3711.0 395.0)) "Undefined" "OverrideRootScale" null null)
    (else
      ;[1 1 1] Common Dialog
      (bind _returnvalue_4 (`|CreateWidget` "/Game/UI/GiantOrc/GiantOrcDialog.GiantOrcDialog_C"))
      (`UserWidget.AddToViewport` _returnvalue_4 0)
      (`WidgetBlueprintLibrary.SetInputMode_UIOnlyEx` _returnvalue _returnvalue_4)
      (`GameplayStatics.SetGamePaused` true)
      (set `PlayerController.bShowMouseCursor` true _returnvalue))))

(fn `UserConstructionScript`)