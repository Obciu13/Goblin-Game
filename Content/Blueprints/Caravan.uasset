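; Caravan loot actor that a GoblinCharacter opens with F while inside its overlap box, which toggles input and a prompt widget.
; The character's CaravanSourgeLevel scales random gold and potion chance, shown through popups and sounds.
; Looting destroys the box and shine components, sets lamp intensity and plays chest animations.
; RandomPotion rerolls for each weighted potion range, so it can grant none or several.
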(event `self.ReceiveBeginPlay`
  (bind (_returnvalue_x _returnvalue_y _returnvalue_z) (`KismetMathLibrary.BreakVector` (`self.K2_GetActorLocation`)))
  (`GameplayStatics.SpawnEmitterAtLocation` "/Game/Geometry/Meshes/Particles/Circle_Particle_Gold.Circle_Particle_Gold" (`KismetMathLibrary.MakeVector` _returnvalue_x _returnvalue_y (+ _returnvalue_z 1.0)) (struct) (1.0 1.0 1.0) false))

(event `Key|F`
  (params (Key :type "Key Structure"))
  (:`Pressed`
    (switch `int` (`/Game/Blueprints/GoblinCharacter.CaravanSourge Level` (`self.As Goblin Character`))
      (:`0`
        ;[1 1 1] Gold Loot
        (`self.Gold Loot` (* (`KismetMathLibrary.RandomIntegerInRange` 2 4) 10))
        ;[1 1 1] Potion Loot
        (set `self.Potion chance` 0.0))
      (:`1`
        (`self.Gold Loot` (* (`KismetMathLibrary.RandomIntegerInRange` 4 6) 10))
        (set `self.Potion chance` 0.3)
        (if (<= (`KismetMathLibrary.RandomFloat`) (`self.Potion chance`)) :!label _label
          (`self.Random Potion`)))
      (:`2`
        (`self.Gold Loot` (* (`KismetMathLibrary.RandomIntegerInRange` 6 8) 10))
        (set `self.Potion chance` 0.6)
        (goto _label))
      (:`3`
        (`self.Gold Loot` (* (`KismetMathLibrary.RandomIntegerInRange` 8 10) 10))
        (set `self.Potion chance` 0.9)
        (goto _label)))
    ;[1 1 1] Loot Animation
    (`ActorComponent.K2_DestroyComponent` (`self.Shine`))
    (`ActorComponent.K2_DestroyComponent` (`self.Shine1`))
    (`ActorComponent.K2_DestroyComponent` (`self.Shine3`))
    (`ActorComponent.K2_DestroyComponent` (`self.Shine4`))
    (`ActorComponent.K2_DestroyComponent` (`self.Shine5`))
    (`ActorComponent.K2_DestroyComponent` (`self.Shine6`))
    (`ActorComponent.K2_DestroyComponent` (`self.Box`))
    (`LightComponent.SetIntensity` (`self.Lamp light`) 300.0)
    (`LightComponent.SetIntensity` (`self.Lamp light1`) 300.0)
    (`SkeletalMeshComponent.PlayAnimation` (`self.chest`) "/Game/Animations/Chest/chest_Anim.chest_Anim" false)
    (`KismetSystemLibrary.Delay` 0.2)
    (`SkeletalMeshComponent.PlayAnimation` (`self.chest1`) "/Game/Animations/Chest/chest_Anim.chest_Anim" false)))

(event `self.Box.OnComponentBeginOverlap`
  (params (OverlappedComponent :type "PrimitiveComponent Object Reference") (OtherActor :type "Actor Object Reference") (OtherComp :type "PrimitiveComponent Object Reference") (OtherBodyIndex :type Integer) (bFromSweep :type Boolean) (SweepResult :type "HitResult Structure (by ref)"))
  ;[1 1 1] Overlap Managment
  (bind _asgoblin_character (cast `/Game/Blueprints/GoblinCharacter` OtherActor))
  (set `self.As Goblin Character` _asgoblin_character)
  (`self.EnableInput` (`GameplayStatics.GetPlayerController` 0))
  (bind _returnvalue (`|CreateWidget` "/Game/UI/Caravan/Caravan_PressF.Caravan_PressF_C"))
  (`UserWidget.AddToViewport` _returnvalue 0))

(event `self.Box.OnComponentEndOverlap`
  (params (OverlappedComponent :type "PrimitiveComponent Object Reference") (OtherActor :type "Actor Object Reference") (OtherComp :type "PrimitiveComponent Object Reference") (OtherBodyIndex :type Integer))
  ;[1 1 1] Overlap Managment
  (cast `/Game/Blueprints/GoblinCharacter` OtherActor)
  (`self.DisableInput` (`GameplayStatics.GetPlayerController` 0))
  (`/Engine/EditorBlueprintResources/StandardMacros.IsValid` (stale `self.Box.OnComponentBeginOverlap` _returnvalue)
    (:`Is Valid`
      (`Widget.RemoveFromParent` (stale `self.Box.OnComponentBeginOverlap` _returnvalue)))))

(event `Random Potion`
  (bind _returnvalue (`KismetMathLibrary.RandomIntegerInRange` 1 15))
  ;[1 1 1] Random Potion
  (`KismetSystemLibrary.Delay` 1.0)
  (`GameplayStatics.PlaySound2D` "/Game/Sounds/Effects/potion_pick_up.potion_pick_up" 1.0 1.0 0.0 null null)
  (`|ExecutionSequence`
    (:`then_0`
      (if (`KismetMathLibrary.InRange_IntInt` _returnvalue 1 5)
        (`/Game/Blueprints/GoblinCharacter.Collect Potion` (`self.As Goblin Character`) "/Game/Blueprints/Potions/Potion_HP.Potion_HP_C")
        (bind _returnvalue_2 (`|CreateWidget` "/Game/UI/CollectPotion_PopUp.CollectPotion_PopUp_C" :!label _label_2))
        (`UserWidget.AddToViewport` _returnvalue_2 0)))
    (:`then_1`
      (if (`KismetMathLibrary.InRange_IntInt` _returnvalue 6 9)
        (`/Game/Blueprints/GoblinCharacter.Collect Potion` (`self.As Goblin Character`) "/Game/Blueprints/Potions/Potion_Of_Speed.Potion_Of_Speed_C")
        (goto _label_2)))
    (:`then_2`
      (if (`KismetMathLibrary.InRange_IntInt` _returnvalue 10 12)
        (`/Game/Blueprints/GoblinCharacter.Collect Potion` (`self.As Goblin Character`) "/Game/Blueprints/Potions/Potion_DashReset.Potion_DashReset_C")
        (goto _label_2)))
    (:`then_3`
      (if (`KismetMathLibrary.InRange_IntInt` _returnvalue 13 14)
        (`/Game/Blueprints/GoblinCharacter.Collect Potion` (`self.As Goblin Character`) "/Game/Blueprints/Potions/Potion_Of_Immunity.Potion_Of_Immunity_C")
        (goto _label_2)))
    (:`then_4`
      (if (`KismetMathLibrary.InRange_IntInt` _returnvalue 15 15)
        (`/Game/Blueprints/GoblinCharacter.Collect Potion` (`self.As Goblin Character`) "/Game/Blueprints/Potions/Potion_Of_Fortune.Potion_Of_Fortune_C")
        (goto _label_2)))))

(fn `Gold Loot`
  (params (Income :type Integer))
  (`/Game/Blueprints/GoblinCharacter.Get Gold` (`self.As Goblin Character`) Income)
  (bind _returnvalue (`|CreateWidget` "/Game/UI/GoldPopUp.GoldPopUp_C"))
  (`UserWidget.AddToViewport` _returnvalue 0)
  (`GameplayStatics.PlaySound2D` "/Game/Sounds/Effects/geld_1.geld_1" 1.0 1.0 0.0 null null))

(fn `UserConstructionScript`)