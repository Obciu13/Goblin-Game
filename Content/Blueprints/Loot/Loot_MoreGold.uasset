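; Gold loot pickup that grants IncomeGold to a GoblinCharacter overlapping its Box.
; Tick uses chained Delays to blink four ShinyGradientTest components on and off.
; On pickup it calls GetGold on the goblin, destroys itself, then shows a GoldPopUp widget.
; The popup's removal sits behind a five-second Delay that follows DestroyActor, so it depends on an already destroyed actor.
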(event `self.ReceiveTick`
  (params (DeltaSeconds :type "Float (single-precision)"))
  (bind _shinygradient_test (`self.ShinyGradient Test`))
  (`KismetSystemLibrary.Delay` 1.0)
  (`SceneComponent.SetVisibility` _shinygradient_test false false)
  (`SceneComponent.SetVisibility` (`self.ShinyGradient Test1`) false false)
  (`SceneComponent.SetVisibility` (`self.ShinyGradient Test2`) false false)
  (`SceneComponent.SetVisibility` (`self.ShinyGradient Test3`) false false)
  (`KismetSystemLibrary.Delay` 0.5)
  (`SceneComponent.SetVisibility` _shinygradient_test true false)
  (`SceneComponent.SetVisibility` (`self.ShinyGradient Test1`) true false)
  (`SceneComponent.SetVisibility` (`self.ShinyGradient Test2`) true false)
  (`SceneComponent.SetVisibility` (`self.ShinyGradient Test3`) true false))

(event `self.box.OnComponentBeginOverlap`
  (params (OverlappedComponent :type "PrimitiveComponent Object Reference") (OtherActor :type "Actor Object Reference") (OtherComp :type "PrimitiveComponent Object Reference") (OtherBodyIndex :type Integer) (bFromSweep :type Boolean) (SweepResult :type "HitResult Structure (by ref)"))
  (bind _asgoblin_character (cast `/Game/Blueprints/GoblinCharacter` OtherActor))
  (`/Game/Blueprints/GoblinCharacter.Get Gold` _asgoblin_character (`self.Income gold`))
  (`self.K2_DestroyActor`)
  (bind _returnvalue (`|CreateWidget` "/Game/UI/GoldPopUp.GoldPopUp_C"))
  (`UserWidget.AddToViewport` _returnvalue 0)
  (`KismetSystemLibrary.Delay` 5.0)
  (`Widget.RemoveFromParent` _returnvalue))

(fn `UserConstructionScript`)