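; Gold loot pickup, apparently dropped by a commander, that pays IncomeGold to the GoblinCharacter that overlaps it.
; BeginPlay spawns a glowing gold emitter at the Cube's location and stores it for cleanup.
; Box overlap plays a coin sound, calls GetGold, destroys the particle and actor, then shows a GoldPopUp widget.
; The popup's timed removal sits on a Delay after DestroyActor, so it likely never runs.
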(event `self.ReceiveBeginPlay`
  (bind _returnvalue (`GameplayStatics.SpawnEmitterAtLocation` "/Game/Geometry/Meshes/Particles/GoldGlowing/GlowingGold_Particle.GlowingGold_Particle" (`SceneComponent.K2_GetComponentLocation` (`self.Cube`)) (struct) (1.0 1.0 1.0) false))
  (set `self.Particle` _returnvalue))

(event `self.box.OnComponentBeginOverlap`
  (params (OverlappedComponent :type "PrimitiveComponent Object Reference") (OtherActor :type "Actor Object Reference") (OtherComp :type "PrimitiveComponent Object Reference") (OtherBodyIndex :type Integer) (bFromSweep :type Boolean) (SweepResult :type "HitResult Structure (by ref)"))
  ;[1 1 1] Collect
  (bind _asgoblin_character (cast `/Game/Blueprints/GoblinCharacter` OtherActor))
  (`GameplayStatics.PlaySound2D` "/Game/Sounds/Effects/geld_1.geld_1" 0.5 1.0 0.0 null null)
  (`/Game/Blueprints/GoblinCharacter.Get Gold` _asgoblin_character (`self.Income gold`))
  (`ActorComponent.K2_DestroyComponent` (`self.Particle`))
  (`self.K2_DestroyActor`)
  (bind _returnvalue (`|CreateWidget` "/Game/UI/GoldPopUp.GoldPopUp_C"))
  (`UserWidget.AddToViewport` _returnvalue 0)
  (`KismetSystemLibrary.Delay` 5.0)
  (`Widget.RemoveFromParent` _returnvalue))

(fn `UserConstructionScript`)