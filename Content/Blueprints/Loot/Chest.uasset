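; Loot chest that a GoblinCharacter can open once for gold, marked by a gold particle circle spawned on BeginPlay.
; Entering the trigger box registers the chest with the goblin and shows an "F to open" widget for up to ten seconds; leaving revokes opening.
; OpenChest plays the animation and sound, grants IncomeGold, then removes the trigger and marker and later replaces the mesh with a brief cloud effect.
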(event `self.ReceiveBeginPlay`
  (bind (_returnvalue_x _returnvalue_y _returnvalue_z) (`KismetMathLibrary.BreakVector` (`SceneComponent.K2_GetComponentLocation` (`self.Box`))))
  (bind _returnvalue (`GameplayStatics.SpawnEmitterAtLocation` "/Game/Geometry/Meshes/Particles/Circle_Particle_Gold.Circle_Particle_Gold" (`KismetMathLibrary.MakeVector` _returnvalue_x _returnvalue_y (- _returnvalue_z 50.0)) (struct) (0.5 0.5 0.5) false)))

(event `self.Box.OnComponentBeginOverlap`
  (params (OverlappedComponent :type "PrimitiveComponent Object Reference") (OtherActor :type "Actor Object Reference") (OtherComp :type "PrimitiveComponent Object Reference") (OtherBodyIndex :type Integer) (bFromSweep :type Boolean) (SweepResult :type "HitResult Structure (by ref)"))
  ;[1 1 1] On Overlap
  (bind _asgoblin_character (cast `/Game/Blueprints/GoblinCharacter` OtherActor))
  (bind _output_get (set `self.As Goblin Character` _asgoblin_character))
  (`/Game/Blueprints/GoblinCharacter.Can Open Chest` _output_get self)
  (bind _returnvalue (`|CreateWidget` "/Game/UI/Chest/Chest_FtoOpen.Chest_FtoOpen_C"))
  (`UserWidget.AddToViewport` _returnvalue 0)
  (`KismetSystemLibrary.Delay` 10.0)
  (`/Engine/EditorBlueprintResources/StandardMacros.IsValid` _returnvalue
    (:`Is Valid`
      (`Widget.RemoveFromParent` _returnvalue))))

(event `self.Box.OnComponentEndOverlap`
  (params (OverlappedComponent :type "PrimitiveComponent Object Reference") (OtherActor :type "Actor Object Reference") (OtherComp :type "PrimitiveComponent Object Reference") (OtherBodyIndex :type Integer))
  ;[1 1 1] On End Overlap
  (bind _asgoblin_character (cast `/Game/Blueprints/GoblinCharacter` OtherActor))
  (`/Game/Blueprints/GoblinCharacter.Cant Open Chest` _asgoblin_character))

(event `Open Chest`
  (bind _skeletalmesh (`self.SkeletalMesh`))
  (bind (_returnvalue_x _returnvalue_y _returnvalue_z) (`KismetMathLibrary.BreakVector` (`SceneComponent.K2_GetComponentLocation` _skeletalmesh)))
  ;[1 1 1] Open Chest
  (`/Engine/EditorBlueprintResources/StandardMacros.DoOnce` false
    (:`Completed`
      (`Widget.RemoveFromParent` (stale `self.Box.OnComponentBeginOverlap` _returnvalue))
      (`SkeletalMeshComponent.PlayAnimation` (`self.SkeletalMesh`) "/Game/Animations/Chest/chest_Anim.chest_Anim" false)
      (`GameplayStatics.PlaySound2D` "/Game/Sounds/Effects/geld_1.geld_1" 1.0 1.0 0.0 null null)
      (`/Game/Blueprints/GoblinCharacter.Get Gold` (`self.As Goblin Character`) (`self.Income Gold`))
      (`ActorComponent.K2_DestroyComponent` (`self.Box`))
      (`ActorComponent.K2_DestroyComponent` (stale `self.ReceiveBeginPlay` _returnvalue))
      (`KismetSystemLibrary.Delay` 2.0)
      (bind _returnvalue (`NiagaraFunctionLibrary.SpawnSystemAtLocation` "/Game/Animations/New_effects/NiagaraSystem/NS_Cloud.NS_Cloud" (`KismetMathLibrary.MakeVector` _returnvalue_x _returnvalue_y _returnvalue_z)))
      (`ActorComponent.K2_DestroyComponent` _skeletalmesh)
      (`KismetSystemLibrary.Delay` 1.0)
      (`ActorComponent.K2_DestroyComponent` _returnvalue))))

(fn `UserConstructionScript`)