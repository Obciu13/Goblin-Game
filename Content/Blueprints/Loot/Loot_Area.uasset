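; Loot area actor that awards gold to the goblin player after they stay inside its capsule for a countdown.
; Overlap registers the area on GoblinCharacter, shortens the wait by its GoldSniffingLevel and shows a countdown widget; leaving resets both.
; A self-calling one-second Delay event ticks the timer down, then grants gold once, plays sound and chest animations, and destroys the capsule and glow particles.
; BeginPlay applies the configured scale and spawns the glows.
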(event `self.ReceiveBeginPlay`
  ;[1 1 1] Scale
  (`self.Scale effect`)
  (bind _returnvalue (`GameplayStatics.SpawnEmitterAtLocation` "/Game/Geometry/Meshes/Particles/GoldGlowing/GlowingGold_Particle.GlowingGold_Particle" (+ (`SceneComponent.K2_GetComponentLocation` (`self.SkeletalMesh1`)) (0.0 0.0 50.0)) (struct) (1.0 1.0 1.0) false))
  (bind _returnvalue_2 (`GameplayStatics.SpawnEmitterAtLocation` "/Game/Geometry/Meshes/Particles/GoldGlowing/GlowingGold_Particle.GlowingGold_Particle" (+ (`SceneComponent.K2_GetComponentLocation` (`self.SkeletalMesh`)) (0.0 0.0 50.0)) (struct) (1.0 1.0 1.0) false)))

(event `self.Capsule.OnComponentBeginOverlap`
  (params (OverlappedComponent :type "PrimitiveComponent Object Reference") (OtherActor :type "Actor Object Reference") (OtherComp :type "PrimitiveComponent Object Reference") (OtherBodyIndex :type Integer) (bFromSweep :type Boolean) (SweepResult :type "HitResult Structure (by ref)"))
  ;[1 1 1] On  Overlap
  (bind _asgoblin_character (cast `/Game/Blueprints/GoblinCharacter` OtherActor))
  (set `/Game/Blueprints/GoblinCharacter.Loot_area` self _asgoblin_character)
  (set `self.Time needed` (- (`self.Time max`) (`KismetMathLibrary.Conv_IntToDouble` (`/Game/Blueprints/GoblinCharacter.GoldSniffing Level` _asgoblin_character))))
  (set `self.Player in range` true)
  (bind _returnvalue (`|CreateWidget` "/Game/UI/Countdown.Countdown_C"))
  (bind _output_get (set `self.Countdown Widget` _returnvalue))
  (`UserWidget.AddToViewport` _output_get 0)
  (`self.Countdown`))

(event `self.Capsule.OnComponentEndOverlap`
  (params (OverlappedComponent :type "PrimitiveComponent Object Reference") (OtherActor :type "Actor Object Reference") (OtherComp :type "PrimitiveComponent Object Reference") (OtherBodyIndex :type Integer))
  ;[1 1 1] On End Overlap
  (bind _asgoblin_character (cast `/Game/Blueprints/GoblinCharacter` OtherActor))
  (set `/Game/Blueprints/GoblinCharacter.Loot_area` null _asgoblin_character)
  (set `self.Player in range` false)
  (set `self.Time needed` (`self.Time max`))
  (if (`KismetSystemLibrary.IsValid` (`self.Countdown Widget`))
    (`Widget.RemoveFromParent` (`self.Countdown Widget`))))

(event `Countdown`
  ;[1 1 1] Countdown
  (`KismetSystemLibrary.Delay` 1.0)
  (if (`self.Player in range`)
    (bind _output_get (set `self.Time needed` (- (`self.Time needed`) (`self.Update rate`))))
    (if (<= _output_get 0.0)
      (bind _asgoblin_character (cast `/Game/Blueprints/GoblinCharacter` (`GameplayStatics.GetPlayerCharacter` 0)))
      (`/Engine/EditorBlueprintResources/StandardMacros.DoOnce` false
        (:`Completed`
          (`/Game/Blueprints/GoblinCharacter.Get Gold` _asgoblin_character (`self.Gold`))
          (set `self.Harvested` true)
          (`Widget.RemoveFromParent` (`self.Countdown Widget`))
          (`GameplayStatics.PlaySound2D` "/Game/Sounds/Effects/geld_1.geld_1" 1.0 1.0 0.0 null null)
          (`SkeletalMeshComponent.PlayAnimation` (`self.SkeletalMesh1`) "/Game/Animations/Chest/chest_Anim.chest_Anim" false)
          (`SkeletalMeshComponent.PlayAnimation` (`self.SkeletalMesh`) "/Game/Animations/Chest/chest_Anim.chest_Anim" false)
          (`KismetSystemLibrary.Delay` 1.0)
          (`ActorComponent.K2_DestroyComponent` (`self.Capsule`))
          (`ActorComponent.K2_DestroyComponent` (`self.Circle_Particle_Gold`))
          (`ActorComponent.K2_DestroyComponent` (stale `self.ReceiveBeginPlay` _returnvalue_2))
          (`ActorComponent.K2_DestroyComponent` (stale `self.ReceiveBeginPlay` _returnvalue))))
      (else
        (`self.Countdown`)))
    (else
      (set `self.Time needed` (`self.Time max`))
      (bind _asgoblin_character_2 (cast `/Game/Blueprints/GoblinCharacter` (`GameplayStatics.GetPlayerCharacter` 0)))
      (set `/Game/Blueprints/GoblinCharacter.Countdown` (`self.Time max`) _asgoblin_character_2))))

(fn `Scale effect`
  ;[1 1 1] Scale effect
  (`SceneComponent.K2_SetWorldTransform` (`self.DefaultSceneRoot`) (`KismetMathLibrary.MakeTransform` (.location (`SceneComponent.K2_GetComponentToWorld` (`self.DefaultSceneRoot`))) (.rotation (`SceneComponent.K2_GetComponentToWorld` (`self.DefaultSceneRoot`))) (`self.Scale`)) false false))

(fn `UserConstructionScript`)