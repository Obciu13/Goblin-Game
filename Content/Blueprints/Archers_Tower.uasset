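; An archer tower that attacks the player's goblin character while it is inside the detection sphere.
; Overlap events toggle an in-range flag and start a self-repeating Shoot loop that turns the bowman, waits, plays the firing animation and spawns AOE arrows.
; Arrows spawn directly near the player rather than at the bow, led along the player's facing direction with random scatter and yawed away from the tower.
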(event `self.ReceiveBeginPlay`
  (`SceneComponent.K2_SetWorldTransform` (`self.bow`) (`SceneComponent.GetSocketTransform` (`self.SkeletalMesh`) "WeaponHold" "RTS_World") false false)
  (`SceneComponent.K2_AttachToComponent` (`self.bow`) (`self.SkeletalMesh`) "WeaponHold" "SnapToTarget" "SnapToTarget" "SnapToTarget" true))

(event `Shoot`
  (bind _skeletalmesh (`self.SkeletalMesh`))
  (bind (_returnvalue_roll _returnvalue_pitch _returnvalue_yaw) (`KismetMathLibrary.BreakRotator` (`KismetMathLibrary.FindLookAtRotation` (`SceneComponent.K2_GetComponentLocation` _skeletalmesh) (`self.K2_GetActorLocation` (`GameplayStatics.GetPlayerCharacter` 0)))))
  ;[1 1 1] Aim and Shoot
  (if (`self.PlayerInRange`)
    (`SceneComponent.K2_SetWorldRotation` _skeletalmesh (`KismetMathLibrary.MakeRotator` 0.0 0.0 (- _returnvalue_yaw 90.0)) false false)
    (`KismetSystemLibrary.Delay` 2.5)
    (`SkeletalMeshComponent.PlayAnimation` (`self.SkeletalMesh`) "/Game/Animations/Bowman/Bowman_shoots.Bowman_shoots" false)
    (bind _returnvalue (`self.Aim For Player`))
    (`|SpawnActorFromClass` "/Game/Blueprints/Skillshots/AOE_Arrows.AOE_Arrows_C" _returnvalue "Undefined" "OverrideRootScale" null null)
    (`self.Shoot`)))

(event `self.Sphere.OnComponentBeginOverlap`
  (params (OverlappedComponent :type "PrimitiveComponent Object Reference") (OtherActor :type "Actor Object Reference") (OtherComp :type "PrimitiveComponent Object Reference") (OtherBodyIndex :type Integer) (bFromSweep :type Boolean) (SweepResult :type "HitResult Structure (by ref)"))
  ;[1 1 1] Check if player in Range
  (cast `/Game/Blueprints/GoblinCharacter` OtherActor)
  (set `self.PlayerInRange` true)
  (`self.Shoot`))

(event `self.Sphere.OnComponentEndOverlap`
  (params (OverlappedComponent :type "PrimitiveComponent Object Reference") (OtherActor :type "Actor Object Reference") (OtherComp :type "PrimitiveComponent Object Reference") (OtherBodyIndex :type Integer))
  ;[1 1 1] Check if player in Range
  (cast `/Game/Blueprints/GoblinCharacter` OtherActor)
  (set `self.PlayerInRange` false))

(fn `Aim For Player`
  (returns (ReturnValue :type "Transform Structure"))
  (bind _returnvalue (`GameplayStatics.GetPlayerCharacter` 0))
  (bind _variety (`self.Variety`))
  (bind _variety_2 (`self.Variety`))
  (return (`KismetMathLibrary.MakeTransform` (+ (`self.K2_GetActorLocation` _returnvalue) (* (`self.GetActorForwardVector` _returnvalue) (`self.distance from character`)) (`KismetMathLibrary.MakeVector` (`KismetMathLibrary.RandomFloatInRange` (* _variety -1.0) _variety) (`KismetMathLibrary.RandomFloatInRange` (* _variety_2 -1.0) _variety_2) 70.0)) (`KismetMathLibrary.MakeRotator` 0.0 0.0 (`KismetMathLibrary.GetYawPitchFromVector` (- (`self.K2_GetActorLocation` (`GameplayStatics.GetPlayerCharacter` 0)) (`self.K2_GetActorLocation`)))))))

(fn `UserConstructionScript`)